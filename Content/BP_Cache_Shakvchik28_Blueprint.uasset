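; BP_Cache_Shakvchik28 is a cache actor that spawns a BP_Boltorez actor attached to itself on BeginPlay.
; The spawned actor takes its scale, local location offset and local rotation from the first BoltorezTransform entry in the BP_GS game state.
; A debug string prints afterwards, and the construction script, overlap and tick events do nothing.
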(event Collision|EventActorBeginOverlap
  (params (OtherActor :type Actor%20Object%20Reference)))

(event EventBeginPlay
  (bind _returnvalue (Game|GetGameState))
  (bind _asbp_gs (Utilities|Casting|CastToBP_GS _returnvalue))
  (bind _boltoreztransform (Variables|/Script/MyProject9.GS|GetBoltorezTransform _asbp_gs))
  (bind _output (Utilities|Array|Get(acopy) _boltoreztransform))
  (bind _returnvalue_2 (Game|SpawnActorfromClass "/Game/Assets/Blueprint/C++_BP/BP_Boltorez.BP_Boltorez_C" (Math|Transform|MakeTransform "0, 0, 0" "0, 0, 0" "1,1,1") "AlwaysSpawn" 0 0))
  (Transformation|AttachActorToActor _returnvalue_2 self "None" "KeepRelative" "KeepRelative" "KeepRelative" true)
  (Transformation|SetActorScale3D _returnvalue_2 (.scale _output))
  (Transformation|AddActorLocalOffset _returnvalue_2 (.location _output) false false)
  (Transformation|AddActorLocalRotation _returnvalue_2 (.rotation _output) false false)
  (Development|PrintString "Hello"))

(event EventTick
  (params (DeltaSeconds :type Float%20%28single-precision%29)))

(fn ConstructionScript)