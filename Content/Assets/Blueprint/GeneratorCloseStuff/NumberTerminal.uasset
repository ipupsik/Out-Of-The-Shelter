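; NumberTerminal is an actor that displays a single digit from 0 to 9 as a decal.
; The construction script switches on NumberType and assigns the matching digit material to the Decal component, so the number is set per instance in the editor.
; The event graph holds only disabled default nodes, so the actor has no runtime logic of its own.
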(event EventBeginPlay)

(event Collision|EventActorBeginOverlap
  (params (OtherActor :type Actor%20Object%20Reference)))

(event EventTick
  (params (DeltaSeconds :type Float%20%28single-precision%29)))

(fn ConstructionScript
  (bind _decal (Variables|Default|GetDecal))
  (switch int (Variables|Default|GetNumberType)
    (:0
      (Rendering|Components|Decal|SetDecalMaterial _decal "/Game/Assets/Blueprint/GeneratorCloseStuff/numbers/0-tra_decal.0-tra_decal"))
    (:1
      (Rendering|Components|Decal|SetDecalMaterial _decal "/Game/Assets/Blueprint/GeneratorCloseStuff/numbers/1-tra_decal.1-tra_decal"))
    (:2
      (Rendering|Components|Decal|SetDecalMaterial _decal "/Game/Assets/Blueprint/GeneratorCloseStuff/numbers/2-tra_decal.2-tra_decal"))
    (:3
      (Rendering|Components|Decal|SetDecalMaterial _decal "/Game/Assets/Blueprint/GeneratorCloseStuff/numbers/3-tra_decal.3-tra_decal"))
    (:4
      (Rendering|Components|Decal|SetDecalMaterial _decal "/Game/Assets/Blueprint/GeneratorCloseStuff/numbers/4-tra_decal.4-tra_decal"))
    (:5
      (Rendering|Components|Decal|SetDecalMaterial _decal "/Game/Assets/Blueprint/GeneratorCloseStuff/numbers/5-tra_decal.5-tra_decal"))
    (:6
      (Rendering|Components|Decal|SetDecalMaterial _decal "/Game/Assets/Blueprint/GeneratorCloseStuff/numbers/6-tra_decal.6-tra_decal"))
    (:7
      (Rendering|Components|Decal|SetDecalMaterial _decal "/Game/Assets/Blueprint/GeneratorCloseStuff/numbers/7-tra_decal.7-tra_decal"))
    (:8
      (Rendering|Components|Decal|SetDecalMaterial _decal "/Game/Assets/Blueprint/GeneratorCloseStuff/numbers/8-tra_decal.8-tra_decal"))
    (:9
      (Rendering|Components|Decal|SetDecalMaterial _decal "/Game/Assets/Blueprint/GeneratorCloseStuff/numbers/9-tra_decal.9-tra_decal"))))