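; ClickButton is a keypad key actor showing a digit, Backspace or Enter decal, chosen from ButtonType in the construction script.
; PlayPressAnim runs a timeline that offsets the Cube's relative Z from its starting position.
; On authority, it also holds ButtonPlayAnim true on the BP_GS game state until the timeline finishes.
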(event Custom|PlayPressAnim
  (bind _asbp_gs (Utilities|Casting|CastToBP_GS (Game|GetGameState)))
  (Networking|SwitchHasAuthority
    (:Authority
      (Variables|/Game/Assets/GameStuff/BP_GS.BP_GS_C|SetButtonPlayAnim _asbp_gs true))
    (:Remote
      _))
  (Variables|Default|SetStartLocation (Variables|/Script/Engine.SceneComponent|GetRelativeLocation (Variables|Default|GetCube)))
  (bind _newtrack_0 (Timeline|Timeline_0 PlayFromStart)
    (:Update
      (Transformation|SetRelativeLocation (Variables|Default|GetCube) (Math|Vector|MakeVector (.X (Math|Vector|BreakVector (Variables|Default|GetStartLocation))) (.Y (Math|Vector|BreakVector (Variables|Default|GetStartLocation))) (+ (.Z (Math|Vector|BreakVector (Variables|Default|GetStartLocation))) _newtrack_0)) false false))
    (:Finished
      (Networking|SwitchHasAuthority
        (:Authority
          (Variables|/Game/Assets/GameStuff/BP_GS.BP_GS_C|SetButtonPlayAnim _asbp_gs false))))))

(fn ConstructionScript
  (bind _decal (Variables|Default|GetDecal))
  (switch int (Variables|Default|GetButtonType)
    (:0
      (Rendering|Components|Decal|SetDecalMaterial _decal "/Game/Assets/Blueprint/GeneratorCloseStuff/numbers/0-tra_decal.0-tra_decal"))
    (:1
      (Rendering|Components|Decal|SetDecalMaterial _decal "/Game/Assets/Blueprint/GeneratorCloseStuff/numbers/1-tra_decal.1-tra_decal"))
    (:2
      (Rendering|Components|Decal|SetDecalMaterial _decal "/Game/Assets/Blueprint/GeneratorCloseStuff/numbers/2-tra_decal.2-tra_decal"))
    (:3
      (Rendering|Components|Decal|SetDecalMaterial _decal "/Game/Assets/Blueprint/GeneratorCloseStuff/numbers/3-tra_decal.3-tra_decal"))
    (:4
      (Rendering|Components|Decal|SetDecalMaterial _decal "/Game/Assets/Blueprint/GeneratorCloseStuff/numbers/4-tra_decal.4-tra_decal"))
    (:5
      (Rendering|Components|Decal|SetDecalMaterial _decal "/Game/Assets/Blueprint/GeneratorCloseStuff/numbers/5-tra_decal.5-tra_decal"))
    (:6
      (Rendering|Components|Decal|SetDecalMaterial _decal "/Game/Assets/Blueprint/GeneratorCloseStuff/numbers/6-tra_decal.6-tra_decal"))
    (:7
      (Rendering|Components|Decal|SetDecalMaterial _decal "/Game/Assets/Blueprint/GeneratorCloseStuff/numbers/7-tra_decal.7-tra_decal"))
    (:8
      (Rendering|Components|Decal|SetDecalMaterial _decal "/Game/Assets/Blueprint/GeneratorCloseStuff/numbers/8-tra_decal.8-tra_decal"))
    (:9
      (Rendering|Components|Decal|SetDecalMaterial _decal "/Game/Assets/Blueprint/GeneratorCloseStuff/numbers/9-tra_decal.9-tra_decal"))
    (:10
      (Rendering|Components|Decal|SetDecalMaterial _decal "/Game/Assets/Blueprint/GeneratorCloseStuff/numbers/backspace-tra_decale.backspace-tra_decale"))
    (:11
      (Rendering|Components|Decal|SetDecalMaterial _decal "/Game/Assets/Blueprint/GeneratorCloseStuff/numbers/enter-tra_decale.enter-tra_decale"))))