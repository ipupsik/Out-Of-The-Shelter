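; A swinging door Blueprint whose Openning event alternately opens and closes it, flipping Switch when each swing finishes.
; Two timelines drive the static mesh's yaw, one played forward and the other in reverse.
; Any overlap with Box1 halts an active swing, and ending the overlap resumes it.
; Overlapping Box sets CanOpenDoor on the MainCh character, and nothing here clears it.
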(event OnComponentBeginOverlap(Box)
  (params (OverlappedComponent :type Primitive%20Component%20Object%20Reference) (OtherActor :type Actor%20Object%20Reference) (OtherComp :type Primitive%20Component%20Object%20Reference) (OtherBodyIndex :type Integer) (bFromSweep :type Boolean) (SweepResult :type Hit%20Result%20Structure%20%28by%20ref%29))
  (bind _asmain_ch (Utilities|Casting|CastToMainCh OtherActor))
  (Variables|/Game/Assets/Characters/MainCh.MainCh_C|SetCanOpenDoor _asmain_ch true))

(event OnComponentBeginOverlap(Box1)
  (params (OverlappedComponent :type Primitive%20Component%20Object%20Reference) (OtherActor :type Actor%20Object%20Reference) (OtherComp :type Primitive%20Component%20Object%20Reference) (OtherBodyIndex :type Integer) (bFromSweep :type Boolean) (SweepResult :type Hit%20Result%20Structure%20%28by%20ref%29))
  (bind _staticmesh (Variables|Default|GetStaticMesh))
  (if (Variables|Default|GetIsPlaying)
    (if (Variables|Default|GetSwitch)
      (bind _z_coord (Timeline|DoorOpening Stop)
        (:Update
          (Transformation|SetRelativeRotation _staticmesh (Math|Rotator|MakeRotator 9e+01 0.0 _z_coord) false false))
        (:Finished
          (Variables|Default|SetSwitch (not (Variables|Default|GetSwitch)) :!label _label)
          (Variables|Default|SetIsPlaying false)))
      (else
        (bind _newtrack_0 (Timeline|DoorOpening_2 Stop)
          (:Update
            (Transformation|SetRelativeRotation _staticmesh (Math|Rotator|MakeRotator 9e+01 0.0 _newtrack_0) false false))
          (:Finished
            (goto _label)))))))

(event OnComponentEndOverlap(Box1)
  (params (OverlappedComponent :type Primitive%20Component%20Object%20Reference) (OtherActor :type Actor%20Object%20Reference) (OtherComp :type Primitive%20Component%20Object%20Reference) (OtherBodyIndex :type Integer))
  (bind _staticmesh (Variables|Default|GetStaticMesh))
  (if (Variables|Default|GetIsPlaying)
    (if (Variables|Default|GetSwitch)
      (bind _z_coord (Timeline|DoorOpening Play)
        (:Update
          (Transformation|SetRelativeRotation _staticmesh (Math|Rotator|MakeRotator 9e+01 0.0 _z_coord) false false))
        (:Finished
          (Variables|Default|SetSwitch (not (Variables|Default|GetSwitch)) :!label _label)
          (Variables|Default|SetIsPlaying false)))
      (else
        (bind _newtrack_0 (Timeline|DoorOpening_2 Reverse)
          (:Update
            (Transformation|SetRelativeRotation _staticmesh (Math|Rotator|MakeRotator 9e+01 0.0 _newtrack_0) false false))
          (:Finished
            (goto _label)))))))

(event Custom|Openning
  (bind _staticmesh (Variables|Default|GetStaticMesh))
  (Variables|Default|SetIsPlaying true)
  (if (Variables|Default|GetSwitch)
    (bind _z_coord (Timeline|DoorOpening PlayFromStart)
      (:Update
        (Transformation|SetRelativeRotation _staticmesh (Math|Rotator|MakeRotator 9e+01 0.0 _z_coord) false false))
      (:Finished
        (Variables|Default|SetSwitch (not (Variables|Default|GetSwitch)) :!label _label)
        (Variables|Default|SetIsPlaying false)))
    (else
      (bind _newtrack_0 (Timeline|DoorOpening_2 ReverseFromEnd)
        (:Update
          (Transformation|SetRelativeRotation _staticmesh (Math|Rotator|MakeRotator 9e+01 0.0 _newtrack_0) false false))
        (:Finished
          (goto _label))))))

(fn ConstructionScript)