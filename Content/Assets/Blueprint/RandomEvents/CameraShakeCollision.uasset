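; A trigger volume that shakes the camera and signals a desaturation effect while the first local player is inside its box.
; Overlap events cast to BP_Player and check that its controller is player controller 0.
; Entering calls the desaturation play hook and starts MyCameraShake, while leaving calls the out hook and stops the shake immediately.
; The desaturation itself is not implemented here, and the post-process dynamic material setup is left unconnected.
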(event OnComponentBeginOverlap(Box)
  (params (OverlappedComponent :type Primitive%20Component%20Object%20Reference) (OtherActor :type Actor%20Object%20Reference) (OtherComp :type Primitive%20Component%20Object%20Reference) (OtherBodyIndex :type Integer) (bFromSweep :type Boolean) (SweepResult :type Hit%20Result%20Structure%20%28by%20ref%29))
  (bind _returnvalue (Game|GetPlayerController 0))
  (bind _asbp_player (Utilities|Casting|CastToBP_Player OtherActor))
  (if (== _returnvalue (Pawn|GetController _asbp_player))
    (Default|CallPlayDusatoration)
    (Class|PlayerController|ClientPlayCameraShake _returnvalue "/Game/Assets/Blueprint/RandomEvents/MyCameraShake.MyCameraShake_C" 1.0 "CameraLocal" "0, 0, 0")))

(event OnComponentEndOverlap(Box)
  (params (OverlappedComponent :type Primitive%20Component%20Object%20Reference) (OtherActor :type Actor%20Object%20Reference) (OtherComp :type Primitive%20Component%20Object%20Reference) (OtherBodyIndex :type Integer))
  (bind _returnvalue (Game|GetPlayerController 0))
  (bind _asbp_player (Utilities|Casting|CastToBP_Player OtherActor))
  (if (== _returnvalue (Pawn|GetController _asbp_player))
    (Default|CallOutplayDesaturation)
    (Game|Feedback|ClientStopCameraShake _returnvalue "/Game/Assets/Blueprint/RandomEvents/MyCameraShake.MyCameraShake_C" true)))

(fn ConstructionScript)