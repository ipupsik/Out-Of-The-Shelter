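; Pedestal Blueprint that tracks how many players stand inside its Box trigger.
; On the server, a begin overlap increments NumberOfPlayers on GameSTATE and an end overlap decrements it, each then calling CheckPlayers.
; Only the decrement requires a MainCh; a failed cast on entry just logs and still increments.
; Debug prints trace overlap start, authority and cast failures.
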(event OnComponentBeginOverlap(Box)
  (params (OverlappedComponent :type Primitive%20Component%20Object%20Reference) (OtherActor :type Actor%20Object%20Reference) (OtherComp :type Primitive%20Component%20Object%20Reference) (OtherBodyIndex :type Integer) (bFromSweep :type Boolean) (SweepResult :type Hit%20Result%20Structure%20%28by%20ref%29))
  (Development|PrintString "Starting Overlap")
  (Networking|SwitchHasAuthority
    (:Authority
      (Utilities|Casting|CastToMainCh OtherActor
        (:then
          _)
        (:CastFailed
          (Development|PrintString "Cast Failed")))
      (bind _asgame_state (Utilities|Casting|CastToGameSTATE (Game|GetGameState))
        (:then
          (Variables|/Game/Assets/GameStuff/GameSTATE.GameSTATE_C|SetNumberOfPlayers _asgame_state (+ (Variables|/Game/Assets/GameStuff/GameSTATE.GameSTATE_C|GetNumberOfPlayers _asgame_state) 1))
          (Default|CheckPlayers _asgame_state)
          (Development|PrintString "PlayersChecked"))
        (:CastFailed
          (Development|PrintString "FailedCastToGameState"))))
    (:Remote
      (Development|PrintString "You have no authority"))))

(event OnComponentEndOverlap(Box)
  (params (OverlappedComponent :type Primitive%20Component%20Object%20Reference) (OtherActor :type Actor%20Object%20Reference) (OtherComp :type Primitive%20Component%20Object%20Reference) (OtherBodyIndex :type Integer))
  (Networking|SwitchHasAuthority
    (:Authority
      (Utilities|Casting|CastToMainCh OtherActor)
      (bind _asgame_state (Utilities|Casting|CastToGameSTATE (Game|GetGameState)))
      (Variables|/Game/Assets/GameStuff/GameSTATE.GameSTATE_C|SetNumberOfPlayers _asgame_state (- (Variables|/Game/Assets/GameStuff/GameSTATE.GameSTATE_C|GetNumberOfPlayers _asgame_state) 1))
      (Default|CheckPlayers _asgame_state))))

(fn ConstructionScript)