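; BP_CanalizationButton is a button Blueprint that animates its mesh sliding along local Y.
; ForwardAnimation and ReverceAnimation relay to matching events named as multicasts, suggesting the motion is meant to play on all networked clients.
; Each direction has its own timeline, played from start for forward and reversed from end for reverse, driving the mesh's relative location.
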(event Custom|Forward%20Multicast
  (bind _y (Timeline|Timeline_0 PlayFromStart)
    (:Update
      (Transformation|SetRelativeLocation (Variables|Character|GetMesh) (Math|Vector|MakeVector 0.0 _y 0.0) false false))))

(event Custom|Reverce%20Multicast
  (bind _y (Timeline|Timeline_1 ReverseFromEnd)
    (:Update
      (Transformation|SetRelativeLocation (Variables|Character|GetMesh) (Math|Vector|MakeVector 0.0 _y 0.0) false false))))

(event EventForwardAnimation
  (CallFunction|ForwardMulticast))

(event EventReverceAnimation
  (CallFunction|ReverceMulticast))

(fn ConstructionScript)