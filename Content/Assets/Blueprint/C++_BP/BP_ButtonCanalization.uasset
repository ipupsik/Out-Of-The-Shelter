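; BP_ButtonCanalization is a button actor that animates by sliding along world X from the position it stores at BeginPlay.
; ForwardAnimation and ReverceAnimation pass through events named as multicasts to play Timeline_0 from the start or reverse it from the end.
; Each timeline update offsets the actor's X by the track value, negated when yaw is positive, so the slide direction follows the actor's facing.
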(event Custom|ReverceMulticast
  (bind _baseposition (Variables|Default|GetBasePosition))
  (bind _newtrack_0 (Timeline|Timeline_0 ReverseFromEnd)
    (:Update
      (if (> (.yaw (Transformation|GetActorRotation)) 0.0)
        (Transformation|SetActorLocation (Math|Vector|MakeVector (+ (.x _baseposition) (* -1 _newtrack_0)) (.y _baseposition) (.z _baseposition)) false false)
        (else
          (Transformation|SetActorLocation (Math|Vector|MakeVector (+ (.x _baseposition) _newtrack_0) (.y _baseposition) (.z _baseposition)) false false))))))

(event Custom|FormardMulticast
  (bind _baseposition (Variables|Default|GetBasePosition))
  (bind _newtrack_0 (Timeline|Timeline_0 PlayFromStart)
    (:Update
      (if (> (.yaw (Transformation|GetActorRotation)) 0.0)
        (Transformation|SetActorLocation (Math|Vector|MakeVector (+ (.x _baseposition) (* -1 _newtrack_0)) (.y _baseposition) (.z _baseposition)) false false)
        (else
          (Transformation|SetActorLocation (Math|Vector|MakeVector (+ (.x _baseposition) _newtrack_0) (.y _baseposition) (.z _baseposition)) false false))))))

(event EventBeginPlay
  (Variables|Default|SetBasePosition (Transformation|GetActorLocation)))

(event EventReverceAnimation
  (CallFunction|ReverceMulticast))

(event EventForwardAnimation
  (CallFunction|FormardMulticast))

(fn ConstructionScript)