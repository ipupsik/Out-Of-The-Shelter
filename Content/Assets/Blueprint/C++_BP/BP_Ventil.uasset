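; BP_Ventil is a valve actor whose mesh turns forward or backward around its roll axis.
; A timeline drives roll from the starting rotation and saves its progress, which also offsets the rotation sound's start time in either direction.
; Multicast events restart or stop that sound and play a separate one-shot gas sound at a given location, with volume scaled by a game-instance audio multiplier.
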(event Custom|SpawnPlaySoundGas_Multicast
  (params (Location :type Vector))
  ;[1 1 1] GasSound
  (Audio|SpawnSoundatLocation "/Game/Assets/Music/partJoined.partJoined" Location "0, 0, 0" (* 0.05 2.0 (Variables|/Game/Assets/GameStuff/BP_GI.BP_GI_C|GetAudioMultiplayer (.AsBP%20GI (Utilities|Casting|CastToBP_GI (Game|GetGameInstance))))) 1.0 0.0 "/Game/Assets/Music/NewSoundAttenuation.NewSoundAttenuation" 0))

(event Custom|PlaySoundStart_Multicast
  ;[1 1 1] Sound ventil
  (Utilities|IsValid (Variables|Default|GetSpawnedRotSound)
    (:Is%20Valid
      (Audio|Components|Audio|Stop (Variables|Default|GetSpawnedRotSound)))
    (:Is%20Not%20Valid
      _))
  (bind _returnvalue (Audio|SpawnSoundatLocation "/Game/Assets/Music/VentilRotationSound.VentilRotationSound" (Transformation|GetActorLocation) "0, 0, 0" (* 0.1 2.0 (Variables|/Game/Assets/GameStuff/BP_GI.BP_GI_C|GetAudioMultiplayer (.AsBP%20GI (Utilities|Casting|CastToBP_GI (Game|GetGameInstance))))) 1.0 (Variables|Default|GetTimeVentilAnim) "/Game/Assets/Music/NewSoundAttenuation.NewSoundAttenuation" 0))
  (Variables|Default|SetSpawnedRotSound _returnvalue))

(event Custom|PlaySoundReverse_Multicast
  ;[1 1 1] Sound ventil
  (Utilities|IsValid (Variables|Default|GetSpawnedRotSound)
    (:Is%20Valid
      (Audio|Components|Audio|Stop (Variables|Default|GetSpawnedRotSound)))
    (:Is%20Not%20Valid
      _))
  (bind _returnvalue (Audio|SpawnSoundatLocation "/Game/Assets/Music/VentilRotationSound.VentilRotationSound" (Transformation|GetActorLocation) "0, 0, 0" (* 0.1 2.0 (Variables|/Game/Assets/GameStuff/BP_GI.BP_GI_C|GetAudioMultiplayer (.AsBP%20GI (Utilities|Casting|CastToBP_GI (Game|GetGameInstance))))) 1.0 (- 1e+01 (Variables|Default|GetTimeVentilAnim)) "/Game/Assets/Music/NewSoundAttenuation.NewSoundAttenuation" 0))
  (Variables|Default|SetSpawnedRotSound _returnvalue))

(event Custom|DestroySound_Multicast
  (bind _spawnedrotsound (Variables|Default|GetSpawnedRotSound))
  ;[1 1 1] Sound ventil
  (Utilities|IsValid _spawnedrotsound
    (:Is%20Valid
      (Audio|Components|Audio|Stop _spawnedrotsound))))

(event Custom|CustomEvent_2
  (params (Location :type Vector))
  ;[1 1 1] GasSound
  (CallFunction|SpawnPlaySoundGasMulticast Location))

(event EventBeginPlay
  (Variables|Default|SetStartingRotation (Transformation|GetActorRotation)))

(event EventRotateVentil
  (bind _startingrotation (Variables|Default|GetStartingRotation))
  (CallFunction|PlaySoundStartMulticast)
  (bind (_direction _rotation _time) (Timeline|Timeline_0 Play)
    (:Update
      (Variables|Default|SetTimeVentilAnim _time)
      (Transformation|SetRelativeRotation (Variables|Character|GetMesh) (Math|Rotator|MakeRotator (+ _rotation (.roll _startingrotation)) (.pitch _startingrotation) (.yaw _startingrotation)) false false))
    (:Finished
      (CallFunction|DestroySoundMulticast))))

(event EventRotateVentilReverse
  (bind _startingrotation (Variables|Default|GetStartingRotation))
  (CallFunction|PlaySoundReverseMulticast)
  (bind (_direction _rotation _time) (Timeline|Timeline_0 Reverse)
    (:Update
      (Variables|Default|SetTimeVentilAnim _time)
      (Transformation|SetRelativeRotation (Variables|Character|GetMesh) (Math|Rotator|MakeRotator (+ _rotation (.roll _startingrotation)) (.pitch _startingrotation) (.yaw _startingrotation)) false false))
    (:Finished
      (CallFunction|DestroySoundMulticast))))

(fn ConstructionScript)