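; Thrown bottle projectile weapon Blueprint that handles hit overlaps and plays a breaking sound.
; Collision begin overlap forwards to OnOverlapBegin, defined outside this graph, then sets DoesHit.
; End overlap acts as a fallback, calling the same handler with a synthesized hit result if DoesHit is still false.
; PlaySoundBroke plays an attenuated sound at the bottle's location, scaled by the game instance's audio multiplier.
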(event OnComponentBeginOverlap(MyCollision)
  (params (OverlappedComponent :type Primitive%20Component%20Object%20Reference) (OtherActor :type Actor%20Object%20Reference) (OtherComp :type Primitive%20Component%20Object%20Reference) (OtherBodyIndex :type Integer) (bFromSweep :type Boolean) (SweepResult :type Hit%20Result%20Structure%20%28by%20ref%29))
  (Class|BottleProjectile|OnOverlapBegin OverlappedComponent OtherActor OtherComp OtherBodyIndex bFromSweep SweepResult)
  (Variables|Default|SetDoesHit true))

(event OnComponentEndOverlap(MyCollision)
  (params (OverlappedComponent :type Primitive%20Component%20Object%20Reference) (OtherActor :type Actor%20Object%20Reference) (OtherComp :type Primitive%20Component%20Object%20Reference) (OtherBodyIndex :type Integer))
  (if (not (Variables|Default|GetDoesHit))
    (Class|BottleProjectile|OnOverlapBegin OverlappedComponent OtherActor OtherComp OtherBodyIndex false (Collision|MakeHitResult false false 0.0 0.0 "0, 0, 0" "0, 0, 0" "0,0,1" "0,0,1" 0 OtherActor))))

(event EventPlaySoundBroke
  (bind _asbp_gi (Utilities|Casting|CastToBP_GI (Game|GetGameInstance)))
  (Audio|SpawnSoundatLocation "/Game/Assets/Music/1.1" (Transformation|GetActorLocation) "0, 0, 0" (* 0.1 2.0 (Variables|/Game/Assets/GameStuff/BP_GI.BP_GI_C|GetAudioMultiplayer _asbp_gi)) 1.0 0.0 "/Game/Assets/Music/NewSoundAttenuationStone.NewSoundAttenuationStone" 0))

(fn ConstructionScript)