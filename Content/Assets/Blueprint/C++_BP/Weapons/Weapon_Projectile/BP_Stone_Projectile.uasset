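; Stone weapon projectile Blueprint that supplies impact sounds for hits on characters ("Chel") and on other objects.
; Each hit event stops the last tracked sound, then spawns an attenuated sound at the projectile, scaled by BP_GI's audio multiplier.
; Character hits play a destruction sound at fixed volume.
; Other hits scale a knock sound by VolumeHit and store it, so the next hit cuts it off.
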(event EventPlaySoundHitChel
  (bind _lastplayedsound (Variables|Default|GetLastPlayedSound))
  (Utilities|IsValid _lastplayedsound
    (:Is%20Valid
      (Audio|Components|Audio|Stop _lastplayedsound))
    (:Is%20Not%20Valid
      _))
  (bind _asbp_gi (Utilities|Casting|CastToBP_GI (Game|GetGameInstance)))
  (Audio|SpawnSoundatLocation "/Game/Assets/Music/Razrushenie.Razrushenie" (Transformation|GetActorLocation) "0, 0, 0" (* 0.1 2.0 (Variables|/Game/Assets/GameStuff/BP_GI.BP_GI_C|GetAudioMultiplayer _asbp_gi)) 1.0 0.0 "/Game/Assets/Music/NewSoundAttenuation.NewSoundAttenuation" 0))

(event EventPlaySoundHitNotChel
  (Utilities|IsValid (Variables|Default|GetLastPlayedSound)
    (:Is%20Valid
      (Audio|Components|Audio|Stop (Variables|Default|GetLastPlayedSound)))
    (:Is%20Not%20Valid
      _))
  (bind _asbp_gi (Utilities|Casting|CastToBP_GI (Game|GetGameInstance)))
  (bind _returnvalue (Audio|SpawnSoundatLocation "/Game/Assets/Music/golf_slabyy_udar_myacha_v_lunku__mp3cut_net_.golf_slabyy_udar_myacha_v_lunku__mp3cut_net_" (Transformation|GetActorLocation) "0, 0, 0" (* (* (Variables|Default|GetvolumeHit) 0.05) 2.0 (Variables|/Game/Assets/GameStuff/BP_GI.BP_GI_C|GetAudioMultiplayer _asbp_gi)) 1.0 0.0 "/Game/Assets/Music/NewSoundAttenuationStone.NewSoundAttenuationStone" 0))
  (Variables|Default|SetLastPlayedSound _returnvalue))

(fn ConstructionScript)