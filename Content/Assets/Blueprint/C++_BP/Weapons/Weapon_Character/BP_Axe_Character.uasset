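; BP_Axe_Character is a character's axe weapon Blueprint that animates the throw and its reverse.
; Two Timelines drive the actor's relative pitch and location without sweep, one for each direction.
; When the throw ends, it plays a stone sound at the axe's location, scaled by the GameInstance audio multiplier, then calls AnimationThrowFinished.
; The reverse animation ends silently by calling AnimationThrowReverseFinished.
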(event EventAnimationThrow
  (bind (_direction _rotation _position) (Timeline|Timeline_1 PlayFromStart)
    (:Update
      (Transformation|SetActorRelativeRotation (Math|Rotator|MakeRotator 0.0 _rotation 0.0))
      (Transformation|SetActorRelativeLocation _position))
    (:Finished
      (bind _asbp_gi (Utilities|Casting|CastToBP_GI (Game|GetGameInstance)))
      (Audio|PlaySoundatLocation "/Game/Assets/Music/StoneMusic1.StoneMusic1" (Transformation|GetActorLocation) "0, 0, 0" (* 0.1 2.0 (Variables|/Game/Assets/GameStuff/BP_GI.BP_GI_C|GetAudioMultiplayer _asbp_gi)) 1.0 0.0 "/Game/Assets/Music/NewSoundAttenuation.NewSoundAttenuation" 0 0)
      (Class|WeaponCharacter|AnimationThrowFinished))))

(event EventAnimationThrowReverse
  (bind (_direction _rotation _position) (Timeline|Timeline_0 PlayFromStart)
    (:Update
      (Transformation|SetActorRelativeRotation (Math|Rotator|MakeRotator 0.0 _rotation 0.0))
      (Transformation|SetActorRelativeLocation _position))
    (:Finished
      (Class|WeaponCharacter|AnimationThrowReverseFinished))))

(fn ConstructionScript)