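; BP_InteractiveCache_Dezinfector is an interactive disinfector cache with a two-stage opening animation.
; Open calls OpenMulticast, which plays a positional sound scaled by the game instance's audio multiplier.
; Chained timelines first slide DopMesh along local Y from its BeginPlay position, then swing the Scene component in yaw.
; Interaction is disabled only once the rotation finishes.
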(event Custom|OpenMulticast
  (bind _dopmesh (Variables|Default|GetDopMesh))
  (bind _relativelocation (Variables|/Script/Engine.SceneComponent|GetRelativeLocation _dopmesh))
  (Audio|PlaySoundatLocation "/Game/Assets/Music/mix_01s__audio-joiner_com___1_.mix_01s__audio-joiner_com___1_" (Transformation|GetWorldLocation (Variables|Default|GetDopMesh)) "0, 0, 0" (* 1.0 2.0 (Variables|/Game/Assets/GameStuff/BP_GI.BP_GI_C|GetAudioMultiplayer (.AsBP%20GI (Utilities|Casting|CastToBP_GI (Game|GetGameInstance))))) 1.0 0.0 "/Game/Assets/Music/NewSoundAttenuation.NewSoundAttenuation" 0 0)
  (bind _newtrack_0 (Timeline|Timeline_1 PlayFromStart)
    (:Update
      (Transformation|SetRelativeLocation _dopmesh (Math|Vector|MakeVector (.x _relativelocation) (+ (Variables|Default|GetStartLocation) _newtrack_0) (.z _relativelocation)) false false))
    (:Finished
      (bind _newtrack_0_2 (Timeline|Timeline_0 PlayFromStart)
        (:Update
          (Transformation|SetRelativeRotation (Variables|Default|GetScene) (Math|Rotator|MakeRotator 0.0 0.0 (* -1 _newtrack_0_2)) false false))
        (:Finished
          (Variables|Default|SetbCanInterract false))))))

(event EventBeginPlay
  (Variables|Default|SetStartLocation (.y (Variables|/Script/Engine.SceneComponent|GetRelativeLocation (Variables|Default|GetDopMesh)))))

(event Collision|EventActorBeginOverlap
  (params (OtherActor :type Actor%20Object%20Reference)))

(event EventTick
  (params (DeltaSeconds :type Float%20%28single-precision%29)))

(event EventOpen
  (CallFunction|OpenMulticast))

(fn ConstructionScript)