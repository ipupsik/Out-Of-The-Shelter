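; BP_Cache_Dezinfector is a cache Blueprint, named as a disinfector, that plays a two-stage opening animation and then cannot be used again.
; Opening calls OpenMulticast to run the animation and immediately clears IsEnabled.
; Timeline_1 slides DopMesh along local Y from the position saved at BeginPlay.
; When that finishes, Timeline_0 swings the Scene component in negative yaw.
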(event Custom|OpenMulticast
  (bind _dopmesh (Variables|Default|GetDopMesh))
  (bind _relativelocation (Variables|/Script/Engine.SceneComponent|GetRelativeLocation _dopmesh))
  (bind _newtrack_0 (Timeline|Timeline_1 PlayFromStart)
    (:Update
      (Transformation|SetRelativeLocation _dopmesh (Math|Vector|MakeVector (.x _relativelocation) (+ (Variables|Default|GetStartLocation) _newtrack_0) (.z _relativelocation)) false false))
    (:Finished
      (bind _newtrack_0_2 (Timeline|Timeline_0 PlayFromStart)
        (:Update
          (Transformation|SetRelativeRotation (Variables|Default|GetScene) (Math|Rotator|MakeRotator 0.0 0.0 (* -1 _newtrack_0_2)) false false))))))

(event EventBeginPlay
  (Variables|Default|SetStartLocation (.y (Variables|/Script/Engine.SceneComponent|GetRelativeLocation (Variables|Default|GetDopMesh)))))

(event EventOpening
  (CallFunction|OpenMulticast)
  (Variables|Default|SetIsEnabled false))

(fn ConstructionScript)