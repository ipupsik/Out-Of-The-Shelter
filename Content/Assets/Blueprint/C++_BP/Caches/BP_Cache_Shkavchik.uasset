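; BP_Cache_Shkavchik is a cache container, apparently a small cabinet, that swings open once triggered.
; Opening calls OpenMulticast, then clears IsEnabled.
; OpenMulticast plays a timeline that drives the yaw of the Scene component to animate the opening.
; Disconnected leftover nodes would spawn and attach a BP_Boltorez using transforms from BP_GS, or set a child actor class, but never run.
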(event Custom|OpenMulticast
  (bind _newtrack_0 (Timeline|Timeline_0 Play)
    (:Update
      (Transformation|SetRelativeRotation (Variables|Default|GetScene) (Math|Rotator|MakeRotator 0.0 0.0 _newtrack_0) false false))))

(event EventBeginPlay)

(event EventOpening
  (CallFunction|OpenMulticast)
  (Variables|Default|SetIsEnabled false))

(fn ConstructionScript)