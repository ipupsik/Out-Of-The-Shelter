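; Interactive loot cache, named as a dumpster (Pomoyka), with an animated opening and a creak sound.
; Open calls OpenMulticast, which plays an attenuated wooden-door creak at the mesh, scaled by the game instance's audio multiplier.
; A timeline rolls the Scene component by its negated track value, then clears CanInterract only once the animation finishes.
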(event Custom|OpenMulticast
  (Audio|PlaySoundatLocation "/Game/Assets/Music/jg-032316-sfx-wood-door-opeining-and-creaking__mp3cut_net___3_.jg-032316-sfx-wood-door-opeining-and-creaking__mp3cut_net___3_" (Transformation|GetWorldLocation (Variables|Character|GetMesh)) "0, 0, 0" (* 0.5 2.0 (Variables|/Game/Assets/GameStuff/BP_GI.BP_GI_C|GetAudioMultiplayer (.AsBP%20GI (Utilities|Casting|CastToBP_GI (Game|GetGameInstance))))) 1.0 0.0 "/Game/Assets/Music/NewSoundAttenuation.NewSoundAttenuation" 0 0)
  (bind _newtrack_0 (Timeline|Timeline_0 Play)
    (:Update
      (Transformation|SetRelativeRotation (Variables|Default|GetScene) (Math|Rotator|MakeRotator (* -1 _newtrack_0) 0.0 0.0) false false))
    (:Finished
      (Variables|Default|SetbCanInterract false))))

(event EventOpen
  (CallFunction|OpenMulticast))

(fn ConstructionScript)