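; Generator area Blueprint that controls the volume of its working ambient sound as the generator state changes.
; Two events forward to multicast events, so the change is meant to play on all clients.
; The working event raises the AmbientWorkingSound volume multiplier by a fixed step on each call, so it accumulates, while the not-working event silences it.
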(event Custom|SoundWorking_Multicast
  (bind _ambientworkingsound (Variables|Default|GetAmbientWorkingSound))
  (bind _audiocomponent (Variables|/Script/Engine.AmbientSound|GetAudioComponent _ambientworkingsound))
  (Audio|Components|Audio|SetVolumeMultiplier _audiocomponent (+ (Variables|/Script/Engine.AudioComponent|GetVolumeMultiplier _audiocomponent) 0.15) :!class /Script/Engine.AudioComponent))

(event Custom|ChangeNotWorking_Multicast
  (Audio|Components|Audio|SetVolumeMultiplier (Variables|/Script/Engine.AmbientSound|GetAudioComponent (Variables|Default|GetAmbientWorkingSound)) 0.0 :!class /Script/Engine.AudioComponent))

(event EventChangeSoundAmbienttoWorking
  (CallFunction|SoundWorkingMulticast))

(event EventChangeSoundAmbienttoNotWorking
  (CallFunction|ChangeNotWorkingMulticast))

(fn ConstructionScript)