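; Valve actor for a gas area, providing multicast sound events for valve rotation and for gas at a given location.
; Rotation sounds replace the previous one and start at an offset from the current turn time, mirrored for reverse, with volume scaled by the game instance's audio multiplier.
; Timeline logic for turning the valve's roll and tracking that time is disconnected, leaving both server rotate events empty.
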(event Custom|SpawnPlaySoundGas_Multicast
  (params (Location :type Vector))
  ;[1 1 1] GasSound
  (Audio|SpawnSoundatLocation "/Game/Assets/Music/partJoined.partJoined" Location "0, 0, 0" (* 0.05 2.0 (Variables|/Game/Assets/GameStuff/BP_GI.BP_GI_C|GetAudioMultiplayer (.AsBP%20GI (Utilities|Casting|CastToBP_GI (Game|GetGameInstance))))) 1.0 0.0 "/Game/Assets/Music/NewSoundAttenuation.NewSoundAttenuation" 0))

(event Custom|PlaySoundStart_Multicast
  ;[1 1 1] Sound ventil
  (Utilities|IsValid (Variables|Default|GetLastSpawnedRotationSound)
    (:Is%20Valid
      (Audio|Components|Audio|Stop (Variables|Default|GetLastSpawnedRotationSound)))
    (:Is%20Not%20Valid
      _))
  (bind _returnvalue (Audio|SpawnSoundatLocation "/Game/Assets/Music/VentilRotationSound.VentilRotationSound" (Transformation|GetActorLocation) "0, 0, 0" (* 0.1 2.0 (Variables|/Game/Assets/GameStuff/BP_GI.BP_GI_C|GetAudioMultiplayer (.AsBP%20GI (Utilities|Casting|CastToBP_GI (Game|GetGameInstance))))) 1.0 (Variables|Default|GetCurTimeVentil) "/Game/Assets/Music/NewSoundAttenuation.NewSoundAttenuation" 0))
  (Variables|Default|SetLastSpawnedRotationSound _returnvalue))

(event Custom|PlaySoundReverse_Multicast
  ;[1 1 1] Sound ventil
  (Utilities|IsValid (Variables|Default|GetLastSpawnedRotationSound)
    (:Is%20Valid
      (Audio|Components|Audio|Stop (Variables|Default|GetLastSpawnedRotationSound)))
    (:Is%20Not%20Valid
      _))
  (bind _returnvalue (Audio|SpawnSoundatLocation "/Game/Assets/Music/VentilRotationSound.VentilRotationSound" (Transformation|GetActorLocation) "0, 0, 0" (* 0.1 2.0 (Variables|/Game/Assets/GameStuff/BP_GI.BP_GI_C|GetAudioMultiplayer (.AsBP%20GI (Utilities|Casting|CastToBP_GI (Game|GetGameInstance))))) 1.0 (- 1e+01 (Variables|Default|GetCurTimeVentil)) "/Game/Assets/Music/NewSoundAttenuation.NewSoundAttenuation" 0))
  (Variables|Default|SetLastSpawnedRotationSound _returnvalue))

(event Custom|DestroySound_Multicast
  (bind _lastspawnedrotationsound (Variables|Default|GetLastSpawnedRotationSound))
  ;[1 1 1] Sound ventil
  (Utilities|IsValid _lastspawnedrotationsound
    (:Is%20Valid
      (Audio|Components|Audio|Stop _lastspawnedrotationsound))))

(event EventRotateVentilServer)

(event EventBeginPlay
  (Variables|Default|SetStartRotation (Transformation|GetActorRotation)))

(event EventRotateVentilServerReverse)

(event EventPlaySoundGas
  (params (Location :type Vector :default "0, 0, 0"))
  ;[1 1 1] GasSound
  (CallFunction|SpawnPlaySoundGasMulticast Location))

(fn ConstructionScript)