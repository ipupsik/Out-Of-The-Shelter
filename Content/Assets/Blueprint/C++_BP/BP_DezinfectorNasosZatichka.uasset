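; Disinfector pump plug actor that animates between an unlocked up state and a locked down state.
; Up and Down events call multicast counterparts, which set the lock and animation-busy flags and play a switch sound scaled by the game instance's audio multiplier.
; A single Offset timeline, played forward or in reverse, slides the plug along local Y and scales the PS component with it, clearing the busy flag when finished.
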(event Custom|SwitchAnimDownMulticast
  (bind _zatichka (Variables|Default|GetZatichka))
  (Variables|Default|SetDoesPlayAnim true)
  (Variables|Default|SetDoesLock true)
  (Audio|PlaySoundatLocation "/Game/Assets/Music/NasosSwitch.NasosSwitch" (Transformation|GetActorLocation) "0, 0, 0" (* 1.0 2.0 (Variables|/Game/Assets/GameStuff/BP_GI.BP_GI_C|GetAudioMultiplayer (.AsBP%20GI (Utilities|Casting|CastToBP_GI (Game|GetGameInstance))))) 1.0 0.0 "/Game/Assets/Music/NewSoundAttenuation.NewSoundAttenuation" 0 0)
  (bind _newtrack_0 (Timeline|Offset ReverseFromEnd)
    (:Update
      (Transformation|SetRelativeLocation _zatichka (Math|Vector|MakeVector 0.0 (* (/ (* 3.596391 _newtrack_0) 1.5) (.x (Variables|/Script/Engine.SceneComponent|GetRelativeScale3D _zatichka))) 0.0) false false)
      (Transformation|SetRelativeScale3D (Variables|Default|GetPS) (Math|Vector|MakeVector (* 0.247219 _newtrack_0) (* 0.247219 _newtrack_0) (* 0.247219 _newtrack_0))))
    (:Finished
      (Variables|Default|SetDoesPlayAnim false))))

(event Custom|SwitchAnimUpMulticast
  (bind _zatichka (Variables|Default|GetZatichka))
  (Variables|Default|SetDoesPlayAnim true)
  (Variables|Default|SetDoesLock false)
  (Audio|PlaySoundatLocation "/Game/Assets/Music/NasosSwitch.NasosSwitch" (Transformation|GetActorLocation) "0,0.000000, 0" (* 1.0 2.0 (Variables|/Game/Assets/GameStuff/BP_GI.BP_GI_C|GetAudioMultiplayer (.AsBP%20GI (Utilities|Casting|CastToBP_GI (Game|GetGameInstance))))) 1.0 0.0 "/Game/Assets/Music/NewSoundAttenuation.NewSoundAttenuation" 0 0)
  (bind _newtrack_0 (Timeline|Offset PlayFromStart)
    (:Update
      (Transformation|SetRelativeLocation _zatichka (Math|Vector|MakeVector 0.0 (* (/ (* 3.596391 _newtrack_0) 1.5) (.x (Variables|/Script/Engine.SceneComponent|GetRelativeScale3D _zatichka))) 0.0) false false)
      (Transformation|SetRelativeScale3D (Variables|Default|GetPS) (Math|Vector|MakeVector (* 0.247219 _newtrack_0) (* 0.247219 _newtrack_0) (* 0.247219 _newtrack_0))))
    (:Finished
      (Variables|Default|SetDoesPlayAnim false))))

(event EventSwitchAnimDown
  (CallFunction|SwitchAnimDownMulticast))

(event EventSwitchAnimUp
  (CallFunction|SwitchAnimUpMulticast))

(fn ConstructionScript)