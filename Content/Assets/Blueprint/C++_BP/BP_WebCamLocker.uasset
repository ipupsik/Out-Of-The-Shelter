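; BP_WebCamLocker is a webcam locker that swings open and closed by rotating its Scene component.
; BeginPlay caches the starting pitch, and a timeline adds its Rotation track to that value, with roll and yaw held fixed.
; Open and Close forward to OpenEverywhere and CloseEverywhere, which play or reverse that timeline.
; DoesPlayAnim is set when either motion starts and cleared when the timeline finishes.
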(event Custom|OpenEverywhere
  (Variables|Default|SetDoesPlayAnim true)
  (bind _rotation (Timeline|Timeline_0 Play)
    (:Update
      (Transformation|SetRelativeRotation (Variables|Default|GetScene) (Math|Rotator|MakeRotator 9e+01 (+ (Variables|Default|GetInitialRotate) _rotation) 0.0) false false))
    (:Finished
      (Variables|Default|SetDoesPlayAnim false))))

(event Custom|CloseEverywhere
  (Variables|Default|SetDoesPlayAnim true)
  (bind _rotation (Timeline|Timeline_0 Reverse)
    (:Update
      (Transformation|SetRelativeRotation (Variables|Default|GetScene) (Math|Rotator|MakeRotator 9e+01 (+ (Variables|Default|GetInitialRotate) _rotation) 0.0) false false))
    (:Finished
      (Variables|Default|SetDoesPlayAnim false))))

(event EventBeginPlay
  (Variables|Default|SetInitialRotate (.pitch (Variables|/Script/Engine.SceneComponent|GetRelativeRotation (Variables|Default|GetScene)))))

(event EventOpen
  (CallFunction|OpenEverywhere))

(event EventClose
  (CallFunction|CloseEverywhere))

(fn ConstructionScript)