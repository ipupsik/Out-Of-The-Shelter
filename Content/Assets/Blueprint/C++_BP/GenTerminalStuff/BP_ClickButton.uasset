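; Clickable button Blueprint, filed with the generator terminal assets, that animates its Item component when pressed.
; ButtonPressAnimation calls a Multicast event, which plays a timeline that offsets Item along relative Z from its starting location.
; The authority sets ButtonPlayAnim on BP_GS when the animation starts and clears it when the timeline finishes, exposing an animation-in-progress flag through the game state.
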(event Custom|Multicast
  (bind _asbp_gs (Utilities|Casting|CastToBP_GS (Game|GetGameState)))
  (Networking|SwitchHasAuthority
    (:Authority
      (Variables|/Script/MyProject9.GS|SetButtonPlayAnim _asbp_gs true))
    (:Remote
      _))
  (Variables|Default|SetStartLocation (Variables|/Script/Engine.SceneComponent|GetRelativeLocation (Variables|Default|GetItem)))
  (bind _newtrack_0 (Timeline|Timeline_0 PlayFromStart)
    (:Update
      (Transformation|SetRelativeLocation (Variables|Default|GetItem) (Math|Vector|MakeVector (.X (Math|Vector|BreakVector (Variables|Default|GetStartLocation))) (.Y (Math|Vector|BreakVector (Variables|Default|GetStartLocation))) (+ (.Z (Math|Vector|BreakVector (Variables|Default|GetStartLocation))) _newtrack_0)) false false))
    (:Finished
      (Networking|SwitchHasAuthority
        (:Authority
          (Variables|/Script/MyProject9.GS|SetButtonPlayAnim _asbp_gs false))))))

(event EventButtonPressAnimation
  (CallFunction|Multicast))

(fn ConstructionScript)