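; BP_ButtonClick is a terminal button Blueprint that animates its mesh when pressed.
; ButtonPressAnimation calls a Multicast event, which caches the mesh's relative location and plays a timeline that offsets it along local Z.
; When the timeline finishes, it sets CanInterract to true.
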(event Custom|Multicast
  (Variables|Default|SetStartLocation (Variables|/Script/Engine.SceneComponent|GetRelativeLocation (Variables|Character|GetMesh)))
  (bind _newtrack_0 (Timeline|Timeline_0 PlayFromStart)
    (:Update
      (Transformation|SetRelativeLocation (Variables|Character|GetMesh) (Math|Vector|MakeVector (.X (Math|Vector|BreakVector (Variables|Default|GetStartLocation))) (.Y (Math|Vector|BreakVector (Variables|Default|GetStartLocation))) (+ (.Z (Math|Vector|BreakVector (Variables|Default|GetStartLocation))) _newtrack_0)) false false))
    (:Finished
      (Variables|Default|SetbCanInterract true))))

(event EventButtonPressAnimation
  (CallFunction|Multicast))

(fn ConstructionScript)