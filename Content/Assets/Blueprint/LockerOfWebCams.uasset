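; LockerOfWebCams is a Blueprint, apparently a webcam locker, that animates opening and closing by rotating its Scene component.
; BeginPlay caches the component's initial pitch as the base angle.
; Open and Close forward to OpenEverywhere and CloseEverywhere, which drive two separate timelines, one played from start and the other reversed from end.
; Each timeline update adds its rotation to the cached pitch, keeping roll and yaw fixed.
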(event Custom|Open
  (CallFunction|OpenEverywhere))

(event Custom|Close
  (CallFunction|CloseEverywhere))

(event Custom|OpenEverywhere
  (bind _rotation (Timeline|Yep PlayFromStart)
    (:Update
      (Transformation|SetRelativeRotation (Variables|Default|GetScene) (Math|Rotator|MakeRotator 9e+01 (+ (Variables|Default|GetInitialRotate) _rotation) 0.0) false false))))

(event Custom|CloseEverywhere
  (bind _rotation (Timeline|Timeline_0 ReverseFromEnd)
    (:Update
      (Transformation|SetRelativeRotation (Variables|Default|GetScene) (Math|Rotator|MakeRotator 9e+01 (+ (Variables|Default|GetInitialRotate) _rotation) 0.0) false false))))

(event EventBeginPlay
  (Variables|Default|SetInitialRotate (.pitch (Variables|/Script/Engine.SceneComponent|GetRelativeRotation (Variables|Default|GetScene)))))

(fn ConstructionScript)