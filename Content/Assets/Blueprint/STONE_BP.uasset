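; STONE_BP is a stone actor that registers hits on MainCh characters, with an Index that exempts characters of the same Index.
; On overlap, only the authority casts the other actor to MainCh and compares indices.
; When they differ, it flags the character for refresh, passes it the stone's Index and calls StonePopadanie.
; The stone then destroys itself through the DeleteStoneAverywhere event.
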(event Custom|DeleteStoneAverywhere
  (Actor|DestroyActor))

(event Collision|EventActorBeginOverlap
  (params (OtherActor :type Actor%20Object%20Reference))
  (Networking|SwitchHasAuthority
    (:Authority
      (bind _asmain_ch (Utilities|Casting|CastToMainCh OtherActor))
      (if (!= (Variables|Default|GetIndex) (Variables|/Game/Assets/Characters/MainCh.MainCh_C|GetIndex _asmain_ch))
        (Variables|/Game/Assets/Characters/MainCh.MainCh_C|SetIsNeedResfresh _asmain_ch true)
        (Variables|/Game/Assets/Characters/MainCh.MainCh_C|SetStoneIndex _asmain_ch (Variables|Default|GetIndex))
        (Default|StonePopadanie _asmain_ch)
        (CallFunction|DeleteStoneAverywhere)))))

(fn ConstructionScript)