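; Exit_Shelter_Opener is a trigger-box Blueprint marking where the player can open the shelter exit.
; On player overlap it sets an in-area flag on MainCh and shows the interface's hold prompt if GameSTATE reports the shelter closed and the player has the key.
; When a MainCh leaves, it clears that flag, hides the prompt, stops interface animations and resets related flags.
; The opening itself is not handled here.
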(event OnComponentBeginOverlap(Box)
  (params (OverlappedComponent :type Primitive%20Component%20Object%20Reference) (OtherActor :type Actor%20Object%20Reference) (OtherComp :type Primitive%20Component%20Object%20Reference) (OtherBodyIndex :type Integer) (bFromSweep :type Boolean) (SweepResult :type Hit%20Result%20Structure%20%28by%20ref%29))
  (if (== (Game|GetPlayerCharacter 0) OtherActor)
    (bind _asmain_ch (Utilities|Casting|CastToMainCh OtherActor))
    (Variables|/Game/Assets/Characters/MainCh.MainCh_C|SetIs_In_Area_Shelter_Opener _asmain_ch true)
    (bind _asgame_state (Utilities|Casting|CastToGameSTATE (Game|GetGameState)))
    (if (and (not (Variables|/Game/Assets/GameStuff/GameSTATE.GameSTATE_C|GetIs_Shelter_Opened _asgame_state)) (Variables|/Game/Assets/Characters/MainCh.MainCh_C|GetHaveKEY _asmain_ch))
      (Utilities|IsValid (Variables|/Game/Assets/Characters/MainCh.MainCh_C|GetInterface _asmain_ch)
        (:Is%20Valid
          (Widget|SetVisibility (Variables|/Game/Assets/UI/UserViewBP.UserViewBP_C|GetHoldText (Variables|/Game/Assets/Characters/MainCh.MainCh_C|GetInterface _asmain_ch)) "Visible"))))))

(event OnComponentEndOverlap(Box)
  (params (OverlappedComponent :type Primitive%20Component%20Object%20Reference) (OtherActor :type Actor%20Object%20Reference) (OtherComp :type Primitive%20Component%20Object%20Reference) (OtherBodyIndex :type Integer))
  (bind _asmain_ch (Utilities|Casting|CastToMainCh OtherActor))
  (Variables|/Game/Assets/Characters/MainCh.MainCh_C|SetIs_In_Area_Shelter_Opener _asmain_ch false)
  (Utilities|IsValid (Variables|/Game/Assets/Characters/MainCh.MainCh_C|GetInterface _asmain_ch)
    (:Is%20Valid
      (Widget|SetVisibility (Variables|/Game/Assets/UI/UserViewBP.UserViewBP_C|GetHoldText (Variables|/Game/Assets/Characters/MainCh.MainCh_C|GetInterface _asmain_ch)) "Hidden")
      (Variables|/Game/Assets/Characters/MainCh.MainCh_C|SetIsStoppedAnimation _asmain_ch true)
      (Class|UserWidget|StopAllAnimations (Variables|/Game/Assets/Characters/MainCh.MainCh_C|GetInterface _asmain_ch))
      (Variables|/Game/Assets/Characters/MainCh.MainCh_C|SetCostil _asmain_ch false))))

(fn ConstructionScript)