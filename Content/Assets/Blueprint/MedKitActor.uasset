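; Rotating med kit pickup that resets a MainCh character's Heath value to zero on overlap and refreshes its percent display.
; Box overlap is handled on the authority, which also clears the character's KIllerIndex.
; Pickup hides the actor and starts a ten-second timer, apparently for Update, which unhides it and immediately applies it to an overlapping character.
; Hiding leaves collision untouched.
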(event OnComponentBeginOverlap(Box)
  (params (OverlappedComponent :type Primitive%20Component%20Object%20Reference) (OtherActor :type Actor%20Object%20Reference) (OtherComp :type Primitive%20Component%20Object%20Reference) (OtherBodyIndex :type Integer) (bFromSweep :type Boolean) (SweepResult :type Hit%20Result%20Structure%20%28by%20ref%29))
  (Networking|SwitchHasAuthority
    (:Authority
      (bind _asmain_ch (Utilities|Casting|CastToMainCh OtherActor))
      (CallFunction|ResizeHealth _asmain_ch)
      (Variables|/Game/Assets/Characters/MainCh.MainCh_C|SetKIllerIndex _asmain_ch -1))))

(event Custom|ResizeHealth
  (params (OverlapedChelick :type Main%20Ch%20Object%20Reference))
  (Variables|/Game/Assets/Characters/MainCh.MainCh_C|SetHeath OverlapedChelick 0.0)
  (Default|SetPercent OverlapedChelick)
  (Rendering|SetActorHiddenInGame true)
  (Utilities|Time|SetTimerbyEvent (EventDispatchers|CreateEvent :!event Update) 1e+01))

(event EventTick
  (params (DeltaSeconds :type Float%20%28single-precision%29))
  (Transformation|AddLocalRotation (Variables|Default|GetScene) (Math|Rotator|MakeRotator 0.0 0.0 (* 100 DeltaSeconds)) false false))

(fn ConstructionScript)

(fn Update
  (Rendering|SetActorHiddenInGame false)
  (bind _array_element (Utilities|Array|ForEachLoopwithBreak (Collision|GetOverlappingActors "/Game/Assets/Characters/MainCh.MainCh_C" :!class /Script/Engine.Actor) :!label _label)
    (:LoopBody
      (bind _asmain_ch (Utilities|Casting|CastToMainCh _array_element))
      (CallFunction|ResizeHealth _asmain_ch)
      (goto _label Break))))