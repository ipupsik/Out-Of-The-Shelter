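; OpenArea is an area actor, apparently a base, for player-openable zones that show UI prompts, but its event logic is disconnected and never runs.
; One chain registers the area and its type on BP_Player, showing UMG_UserView's hold or area-used text according to IsAvaliable.
; The other clears those references, hides both texts and stops widget animations.
; The construction script and DoSomethink are empty.
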(fn ConstructionScript)

(fn DoSomethink)