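; GasArea_Damage is a gas zone actor that doubles the player's radiation coefficient while they are inside its Box volume.
; On overlap begin it casts to BP_Player, shows the double radiation effect on the player's UMG_UserView and multiplies RadCoeff by two.
; On overlap end it disables the effect and halves RadCoeff, both only when the UI widget is valid.
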(event OnComponentBeginOverlap(Box)
  (params (OverlappedComponent :type Primitive%20Component%20Object%20Reference) (OtherActor :type Actor%20Object%20Reference) (OtherComp :type Primitive%20Component%20Object%20Reference) (OtherBodyIndex :type Integer) (bFromSweep :type Boolean) (SweepResult :type Hit%20Result%20Structure%20%28by%20ref%29))
  (bind _asbp_player (Utilities|Casting|CastToBP_Player OtherActor))
  (bind _asumg_user_view (Utilities|Casting|CastToUMG_UserView (Variables|/Script/MyProject9.Chel|GetUserView _asbp_player)))
  (Utilities|IsValid _asumg_user_view
    (:Is%20Valid
      (Default|AddDoubleRadiationEffect _asumg_user_view)
      (Variables|/Script/MyProject9.Chel|SetRadCoeff _asbp_player (* (Variables|/Script/MyProject9.Chel|GetRadCoeff _asbp_player) 2.0)))))

(event OnComponentEndOverlap(Box)
  (params (OverlappedComponent :type Primitive%20Component%20Object%20Reference) (OtherActor :type Actor%20Object%20Reference) (OtherComp :type Primitive%20Component%20Object%20Reference) (OtherBodyIndex :type Integer))
  (bind _asbp_player (Utilities|Casting|CastToBP_Player OtherActor))
  (bind _asumg_user_view (Utilities|Casting|CastToUMG_UserView (Variables|/Script/MyProject9.Chel|GetUserView _asbp_player)))
  (Utilities|IsValid _asumg_user_view
    (:Is%20Valid
      (Default|DisableDoubleRadiationEffect _asumg_user_view)
      (Variables|/Script/MyProject9.Chel|SetRadCoeff _asbp_player (* (Variables|/Script/MyProject9.Chel|GetRadCoeff _asbp_player) 0.5)))))

(fn ConstructionScript)