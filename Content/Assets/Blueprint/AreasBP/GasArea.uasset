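; Gas area interactable, built on a parent area class, that temporarily releases gas and damage zones when triggered.
; DoSomethink marks it unavailable, updates overlapping players' hold prompts, and spawns gas and damage actors at tagged TargetPoints, stamping each with its tag.
; After a fixed delay it becomes available again and destroys only spawned actors matching those tags.
; It then restores the hold prompt for eligible players still overlapping.
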(event EventBeginPlay
  (|CallParentFunction)
  (Variables|Default|SetCurrentAreaType (Variables|Default|GetAreaType)))

(event Collision|EventActorBeginOverlap
  (params (OtherActor :type Actor%20Object%20Reference))
  (|CallParentFunction OtherActor) ; This node is disabled and will not be called.\nDrag off pins to build functionality.
)

(event EventTick
  (params (DeltaSeconds :type Float%20%28single-precision%29))
  (|CallParentFunction DeltaSeconds) ; This node is disabled and will not be called.\nDrag off pins to build functionality.
)

(event EventDoSomethink
  (Development|PrintString "In Gas Area Do Somethink Function")
  (Variables|Default|SetIsAvaliable false)
  (for _array_element (Collision|GetOverlappingActors "/Game/Assets/Characters/BP_Player.BP_Player_C" :!class /Script/Engine.Actor)
    (bind _asbp_player (Utilities|Casting|CastToBP_Player _array_element))
    (Variables|/Game/Assets/Characters/BP_Player.BP_Player_C|SetIsOpenWasSuccesfly _asbp_player false)
    (bind _asumg_user_view (Utilities|Casting|CastToUMG_UserView (Variables|/Script/MyProject9.Chel|GetUserView _asbp_player)))
    (Utilities|IsValid _asumg_user_view
      (:Is%20Valid
        (Widget|SetVisibility (Variables|/Script/MyProject9.UserView|GetHoldText _asumg_user_view) "Hidden")
        (Widget|SetVisibility (Variables|Default|GetAreaUsedText _asumg_user_view) "Visible")
        (Class|UserWidget|StopAnimation _asumg_user_view (Variables|Default|GetOpenAreaAnim _asumg_user_view)))))
  (bind _outactors (Actor|GetAllActorsOfClasswithTag "/Script/Engine.TargetPoint" (Utilities|String|StringToName (Variables|Default|GetTargetPointTag))))
  (for _array_element_2 _outactors
    (bind _returnvalue (Game|SpawnActorfromClass (Variables|Default|GetGasClass) (Transformation|GetActorTransform _array_element_2) "Undefined" 0 0))
    (Variables|/Game/Assets/ParticleSystem/ParticleGas.ParticleGas_C|SetAreaType _returnvalue (Variables|Default|GetTargetPointTag)))
  (bind _outactors_2 (Actor|GetAllActorsOfClasswithTag "/Script/Engine.TargetPoint" (Utilities|String|StringToName (Variables|Default|GetGasAreaDamageTag))))
  (for _array_element_3 _outactors_2
    (bind _returnvalue_2 (Game|SpawnActorfromClass (Variables|Default|GetGasDamageAreaClass) (Transformation|GetActorTransform _array_element_3) "Undefined" 0 0))
    (Variables|/Game/Assets/Blueprint/AreasBP/GasArea_Damage.GasArea_Damage_C|SetAreaType _returnvalue_2 (Variables|Default|GetGasAreaDamageTag)))
  (Utilities|FlowControl|Delay 2e+01)
  (Variables|Default|SetIsAvaliable true)
  (bind _outactors_3 (Actor|GetAllActorsOfClass (Variables|Default|GetGasClass)))
  (for _array_element_4 _outactors_3
    (if (Utilities|Enum|Equal(Enum) (Variables|/Game/Assets/ParticleSystem/ParticleGas.ParticleGas_C|GetAreaType _array_element_4) (Variables|Default|GetTargetPointTag))
      (Actor|DestroyActor _array_element_4)))
  (bind _outactors_4 (Actor|GetAllActorsOfClass (Variables|Default|GetGasDamageAreaClass)))
  (for _array_element_5 _outactors_4
    (if (Utilities|Enum|Equal(Enum) (Variables|/Game/Assets/Blueprint/AreasBP/GasArea_Damage.GasArea_Damage_C|GetAreaType _array_element_5) (Variables|Default|GetGasAreaDamageTag))
      (Actor|DestroyActor _array_element_5)))
  (for _array_element_6 (Collision|GetOverlappingActors "/Game/Assets/Characters/BP_Player.BP_Player_C" :!class /Script/Engine.Actor)
    (bind _asbp_player_2 (Utilities|Casting|CastToBP_Player _array_element_6))
    (bind _asumg_user_view_2 (Utilities|Casting|CastToUMG_UserView (Variables|/Script/MyProject9.Chel|GetUserView _asbp_player_2)))
    (if (and (Utilities|Enum|Equal(Enum) (Variables|/Game/Assets/Characters/BP_Player.BP_Player_C|GetTypeOpenArea _asbp_player_2) (Variables|Default|GetAreaType)) (Variables|/Game/Assets/Blueprint/AreasBP/OpenArea.OpenArea_C|GetIsAvaliable (Variables|/Game/Assets/Characters/BP_Player.BP_Player_C|GetOpenAreaObj _asbp_player_2)))
      (Utilities|IsValid _asumg_user_view_2
        (:Is%20Valid
          (Widget|SetVisibility (Variables|Default|GetAreaUsedText _asumg_user_view_2) "Hidden")
          (Widget|SetVisibility (Variables|/Script/MyProject9.UserView|GetHoldText _asumg_user_view_2) "Visible"))))))

(fn ConstructionScript
  (|CallParentFunction))