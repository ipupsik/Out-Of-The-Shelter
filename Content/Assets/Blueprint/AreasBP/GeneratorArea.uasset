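; GeneratorArea is a single-use interaction zone for a generator, detected through a collision overlap.
; On entry it registers itself as the BP_Player's GenAreaObj and shows either a hold prompt or an area-used message, depending on IsAvaliable.
; On exit it clears that reference, hides both texts and deletes the player's generator widget.
; DoSomethinkGen is a placeholder action that prints a debug string and marks the area unavailable.
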(event OnComponentBeginOverlap(Collision)
  (params (OverlappedComponent :type Primitive%20Component%20Object%20Reference) (OtherActor :type Actor%20Object%20Reference) (OtherComp :type Primitive%20Component%20Object%20Reference) (OtherBodyIndex :type Integer) (bFromSweep :type Boolean) (SweepResult :type Hit%20Result%20Structure%20%28by%20ref%29))
  (bind _asbp_player (Utilities|Casting|CastToBP_Player OtherActor))
  (Variables|/Game/Assets/Characters/BP_Player.BP_Player_C|SetGenAreaObj _asbp_player self)
  (if (Variables|Default|GetIsAvaliable)
    (Widget|SetVisibility (Variables|/Script/MyProject9.UserView|GetHoldText (Variables|/Script/MyProject9.Chel|GetUserView _asbp_player)) "Visible")
    (else
      (Utilities|IsValid (Variables|/Script/MyProject9.Chel|GetUserView _asbp_player)
        (:Is%20Valid
          (Widget|SetVisibility (Variables|/Script/MyProject9.UserView|GetAreaUsedText (Variables|/Script/MyProject9.Chel|GetUserView _asbp_player)) "Visible"))))))

(event OnComponentEndOverlap(Collision)
  (params (OverlappedComponent :type Primitive%20Component%20Object%20Reference) (OtherActor :type Actor%20Object%20Reference) (OtherComp :type Primitive%20Component%20Object%20Reference) (OtherBodyIndex :type Integer))
  (bind _asbp_player (Utilities|Casting|CastToBP_Player OtherActor))
  (Variables|/Game/Assets/Characters/BP_Player.BP_Player_C|SetGenAreaObj _asbp_player 0)
  (Utilities|IsValid (Variables|/Script/MyProject9.Chel|GetUserView _asbp_player)
    (:Is%20Valid
      (Widget|SetVisibility (Variables|/Script/MyProject9.UserView|GetAreaUsedText (Variables|/Script/MyProject9.Chel|GetUserView _asbp_player)) "Hidden")
      (Default|DeleteGeneratorWidget _asbp_player)
      (Widget|SetVisibility (Variables|/Script/MyProject9.UserView|GetHoldText (Variables|/Script/MyProject9.Chel|GetUserView _asbp_player)) "Hidden"))))

(event Custom|DoSomethinkGen
  (Development|PrintString "Krasava")
  (Variables|Default|SetIsAvaliable false))

(fn ConstructionScript)