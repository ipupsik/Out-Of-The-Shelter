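; CanalizationDamageArea is a sewer radiation area with a Box volume and logic for setting BP_Player's AddRadiation, but none of its chains has a triggering event.
; Two authority-only chains would apply or clear RadiationDamage on a player.
; A shutdown chain would zero radiation, start a timer and disable GovnoCanalizaciaButton refresh.
; A restore chain would reset the damage rate, zero overlapping players' radiation, re-enable refresh and close the buttons.
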(fn ConstructionScript)