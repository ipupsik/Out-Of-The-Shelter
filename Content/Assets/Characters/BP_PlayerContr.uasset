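; Multiplayer player controller that handles the Escape menu, music, post-process outline toggle and session leaving.
; On BeginPlay the first local controller starts hub music and creates the menu, which switches input mode and flags the pawn.
; For the winners scene, it passes saved cosmetics from BP_GI to spawn a character using BP_GS results.
; When leaving, a host tears down other controllers' sessions, while others update vote counts or reset the game.
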(event Custom|DecreaseAmount
  (bind _asbp_gs (Utilities|Casting|CastToBP_GS (Game|GetGameState)))
  (bind _output_get (Variables|/Script/MyProject9.GS|SetAmountOfPlayers _asbp_gs (- (Variables|/Script/MyProject9.GS|GetAmountOfPlayers _asbp_gs) 1)))
  (if (Variables|Default|GetIsHost)
    (bind _outactors (Actor|GetAllActorsOfClass "BP_PlayerContr_C"))
    (for _array_element _outactors
      (if (!= _array_element self)
        (CallFunction|DestroySession _array_element)))
    (else
      (CallFunction|DestroyClient)
      (if (== _output_get (Variables|/Script/MyProject9.GS|GetAgreedPlayers _asbp_gs))
        (Class|GS|ResetGame (Variables|Default|GetGS))
        (Class|BPPlayerController|RemoveFinalMenu))
      (bind _outactors_2 (Actor|GetAllActorsOfClass "BP_PlayerContr_C"))
      (for _array_element_2 _outactors_2
        (Class|BPPlayerController|RefreshPlayersVoteCount _array_element_2 (Variables|/Script/MyProject9.GS|GetAgreedPlayers _asbp_gs) _output_get)))))

(event Custom|DestroySession
  (bind _asbp_gi (Utilities|Casting|CastToBP_GI (Game|GetGameInstance)))
  (Default|DestroyServer _asbp_gi self)
  (CallFunction|IsAlready))

(event Custom|IsAlready
  (bind _result (Math|Integer|DecrementInt (Variables|/Script/MyProject9.GS|GetAmountOfPlayers (Variables|Default|GetGS)))
    (:%20%20
      (if (== 1 _result)
        (bind _asbp_gi (Utilities|Casting|CastToBP_GI (Game|GetGameInstance)))
        (Default|DestroyServer _asbp_gi self)))))

(event Custom|DestroyClient
  (bind _asbp_gi (Utilities|Casting|CastToBP_GI (Game|GetGameInstance)))
  (Default|DestroyServer _asbp_gi self))

(event Custom|GetCustomizationPreset
  (params (Index :type Integer))
  (bind _asbp_gi (Utilities|Casting|CastToBP_GI (Game|GetGameInstance)))
  (Audio|Components|Audio|Stop (Variables|Default|GetGameplayMusic))
  (bind _returnvalue (Audio|SpawnSound2D "/Game/Assets/Music/Among_The_Stars_-_AShamaluevMusic__mp3cut_net__Cue.Among_The_Stars_-_AShamaluevMusic__mp3cut_net__Cue" (* 1.0 2.0 (Variables|/Game/Assets/GameStuff/BP_GI.BP_GI_C|GetAudioMultiplayer _asbp_gi)) 1.0 0.0 0))
  (Variables|Default|SetWinnersMusic _returnvalue)
  (CallFunction|DeliverPresettoServer (Variables|/Game/Assets/GameStuff/BP_GI.BP_GI_C|GetPrevHat _asbp_gi) (Variables|/Game/Assets/GameStuff/BP_GI.BP_GI_C|GetPrevAccesori _asbp_gi) (Variables|/Game/Assets/GameStuff/BP_GI.BP_GI_C|GetPrevShirt _asbp_gi) (Variables|/Game/Assets/GameStuff/BP_GI.BP_GI_C|GetPrevTShirt _asbp_gi) Index))

(event Custom|DeliverPresetToServer
  (params (Hat :type Items%20Customization%20Struct%20Structure) (Accesori :type Items%20Customization%20Struct%20Structure) (Shirt :type Items%20Customization%20Struct%20Structure) (TShirt :type Items%20Customization%20Struct%20Structure) (Index :type Integer))
  (bind _asbp_gs (Utilities|Casting|CastToBP_GS (Game|GetGameState)))
  (Game|SpawnActorfromClass "/Game/Assets/Characters/CustomizationChel.CustomizationChel_C" (Utilities|Array|Get(acopy) (Variables|/Game/Assets/GameStuff/BP_GS.BP_GS_C|GetPlayersTransform _asbp_gs) Index) "Undefined" 0 Hat Accesori Shirt TShirt true (Utilities|Array|Get(acopy) (Variables|/Script/MyProject9.GS|GetWinnersNickNames _asbp_gs) Index) (Utilities|Array|Get(acopy) (Variables|/Script/MyProject9.GS|GetEscapeTime _asbp_gs) Index) 0))

(event Custom|EnableOutlineClient
  (bind _outactors (Actor|GetAllActorsOfClass "/Script/Engine.PostProcessVolume"))
  (Utilities|Array|SetArrayElem (Utilities|Struct|BreakWeightedBlendables (Utilities|Struct|BreakPostProcessSettings (Variables|/Script/Engine.PostProcessVolume|GetSettings (Utilities|Array|Get(acopy) _outactors)))) 0 (Utilities|Struct|MakeWeightedBlendable 1.0 (.Object (Utilities|Struct|BreakWeightedBlendable (Utilities|Array|Get(acopy) (Utilities|Struct|BreakWeightedBlendables (Utilities|Struct|BreakPostProcessSettings (Variables|/Script/Engine.PostProcessVolume|GetSettings (Utilities|Array|Get(acopy) _outactors))))))))))

(event Custom|DissableOutlineClient
  (bind _outactors (Actor|GetAllActorsOfClass "/Script/Engine.PostProcessVolume"))
  (Utilities|Array|SetArrayElem (Utilities|Struct|BreakWeightedBlendables (Utilities|Struct|BreakPostProcessSettings (Variables|/Script/Engine.PostProcessVolume|GetSettings (Utilities|Array|Get(acopy) _outactors)))) 0 (Utilities|Struct|MakeWeightedBlendable 0.0 (.Object (Utilities|Struct|BreakWeightedBlendable (Utilities|Array|Get(acopy) (Utilities|Struct|BreakWeightedBlendables (Utilities|Struct|BreakPostProcessSettings (Variables|/Script/Engine.PostProcessVolume|GetSettings (Utilities|Array|Get(acopy) _outactors))))))))))

(event EventBeginPlay
  (bind _asbp_gi (Utilities|Casting|CastToBP_GI (Game|GetGameInstance)))
  (if (== (Game|GetPlayerController 0) self)
    (bind _returnvalue (Audio|SpawnSound2D "/Game/Assets/Music/Melody/HubMusic__online-audio-converter_com__Cue.HubMusic__online-audio-converter_com__Cue" (* 0.1 2.0 (Variables|/Game/Assets/GameStuff/BP_GI.BP_GI_C|GetAudioMultiplayer _asbp_gi)) 1.0 0.0 0))
    (Variables|Default|SetHubMusic _returnvalue)
    (bind _returnvalue_2 (UserInterface|CreateWidget "/Game/Assets/UI/EscMenu.EscMenu_C" self))
    (bind _output_get (Variables|Default|SetEscWidget _returnvalue_2))
    (UserInterface|Viewport|AddtoViewport _output_get 20)
    (Widget|SetVisibility _output_get "Hidden")))

(event EventDisableOutline
  (CallFunction|DissableOutlineClient))

(event EventEnableOutline
  (CallFunction|EnableOutlineClient))

(event EventPlayGameplayMusic
  (Audio|Components|Audio|Stop (Variables|Default|GetHubMusic))
  (bind _asbp_gi (Utilities|Casting|CastToBP_GI (Game|GetGameInstance)))
  (bind _returnvalue (Audio|SpawnSound2D "/Game/Assets/Music/Melody/Hi-Tech_Background_Theme__online-audio-converter_com__Cue.Hi-Tech_Background_Theme__online-audio-converter_com__Cue" (* 0.005 2.0 (Variables|/Game/Assets/GameStuff/BP_GI.BP_GI_C|GetAudioMultiplayer _asbp_gi)) 1.0 0.0 0))
  (Variables|Default|SetGameplayMusic _returnvalue))

(event Input|KeyboardEvents|Escape
  (params (Key :type Key%20Structure :default "None"))
  (bind _returnvalue (Pawn|GetControlledPawn))
  (bind _self self)
  (bind _escwidget (Variables|Default|GetEscWidget))
  (:Pressed
    (if (Widget|IsVisible (Variables|Default|GetEscWidget))
      (Widget|SetVisibility _escwidget "Hidden")
      (Input|SetInputModeGameOnly _self)
      (Variables|/Script/Engine.PlayerController|SetbShowMouseCursor _self false)
      (Default|RefreshEscMenu (Variables|Default|GetEscWidget))
      (bind _asbp_player (Utilities|Casting|CastToBP_Player _returnvalue))
      (Variables|/Script/MyProject9.Chel|SetbInEscMenu _asbp_player false)
      (else
        (Widget|SetVisibility _escwidget "Visible")
        (Input|SetInputModeGameandUI self _escwidget "DoNotLock" false)
        (Variables|/Script/Engine.PlayerController|SetbShowMouseCursor _self true)
        (bind _asbp_player_2 (Utilities|Casting|CastToBP_Player _returnvalue))
        (Variables|/Script/MyProject9.Chel|SetbInEscMenu _asbp_player_2 true)))))

(fn ConstructionScript)