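; Main-menu version of the player pawn that shows the menu through BP_GI and animates the menu's camera transitions.
; Open plays a timeline that raises the Menu_Door mesh, moves and turns the pawn, and drives the menu's opacity before removing it.
; A second timeline moves the pawn and camera yaw into customization and reverses to return.
; LookRight spins the CustomizationChel actor once ThrowStone is pressed on menu page 4; Escape forwards to the menu.
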(event Custom|Open
  (bind _startlocationchel (Variables|Default|GetStartLocationChel))
  (bind _startlocationdoor (Variables|Default|GetStartLocationDoor))
  (bind (_direction _up _newtrack_1 _x_offset _y_offset _menu_opacity) (Timeline|Timeline_0 PlayFromStart)
    (:Update
      (Transformation|SetActorLocation (Variables|/Game/Assets/Blueprint/Menu_Door.Menu_Door_C|GetStaticMesh (Variables|Default|GetMenuDoor)) (Math|Vector|MakeVector (.x _startlocationdoor) (.y _startlocationdoor) (+ _up (.z _startlocationdoor))) false false)
      (Transformation|SetActorRotation (Math|Rotator|MakeRotator 0.0 0.0 _newtrack_1))
      (Transformation|SetActorLocation (Math|Vector|MakeVector (+ _x_offset (.x _startlocationchel)) (+ _y_offset (.y _startlocationchel)) (.z _startlocationchel)) false false)
      (Widget|SetRenderOpacity (Variables|Default|GetMainMenu) _menu_opacity))
    (:Finished
      (Widget|RemovefromParent (Variables|Default|GetMainMenu)))))

(event Custom|GoToCutomization
  (bind (_direction _newtrack_1 _newtrack_0) (Timeline|Customization Play)
    (:Update
      (Transformation|SetActorLocation (+ (Variables|Default|GetStartLocationChel) _newtrack_0) false false)
      (Transformation|SetRelativeRotation (Variables|Default|GetCamera) (Math|Rotator|MakeRotator 0.0 0.0 _newtrack_1) false false))))

(event Custom|BackCustomization
  (bind (_direction _newtrack_1 _newtrack_0) (Timeline|Customization Reverse)
    (:Update
      (Transformation|SetActorLocation (+ (Variables|Default|GetStartLocationChel) _newtrack_0) false false)
      (Transformation|SetRelativeRotation (Variables|Default|GetCamera) (Math|Rotator|MakeRotator 0.0 0.0 _newtrack_1) false false))))

(event EventBeginPlay
  (bind _asbp_gi (Utilities|Casting|CastToBP_GI (Game|GetGameInstance)))
  (Default|ShowMainMenu _asbp_gi)
  (bind _outactors (Actor|GetAllActorsOfClass "/Game/Assets/Blueprint/Menu_Door.Menu_Door_C"))
  (bind _output_get (Variables|Default|SetMenuDoor (Utilities|Array|Get(acopy) _outactors)))
  (Variables|Default|SetStartLocationDoor (Transformation|GetActorLocation (Variables|/Game/Assets/Blueprint/Menu_Door.Menu_Door_C|GetStaticMesh _output_get)))
  (Variables|Default|SetStartLocationChel (Transformation|GetActorLocation))
  (bind _outactors_2 (Actor|GetAllActorsOfClass "/Game/Assets/Characters/CustomizationChel.CustomizationChel_C"))
  (Variables|Default|SetCustomizationMesh (Utilities|Array|Get(acopy) _outactors_2)))

(event EventTick
  (params (DeltaSeconds :type Float%20%28single-precision%29)))

(event Input|ActionEvents|InputActionThrowStone
  (params (Key :type Key%20Structure :default "None"))
  (:Pressed
    (if (== (Variables|/Script/UMG.WidgetSwitcher|GetActiveWidgetIndex (Variables|/Game/Assets/UI/UMG_MainMenu.UMG_MainMenu_C|GetWidgetSwitcher_121 (Variables|Default|GetMainMenu))) 4)
      (Variables|Default|SetDoesRotate true)
      (else
        (Variables|Default|SetDoesRotate false)))))

(event Input|AxisEvents|InputAxisLookRight
  (params (AxisValue :type Float%20%28single-precision%29))
  (if (Variables|Default|GetDoesRotate)
    (Class|Actor|AddActorWorldRotation (Variables|Default|GetCustomizationMesh) (Math|Rotator|MakeRotator 0.0 0.0 (* AxisValue (Variables|Default|GetRotateSpeed) -1.0)))))

(event Input|KeyboardEvents|Escape
  (params (Key :type Key%20Structure :default "None"))
  (:Pressed
    (Default|EscapeMenu (Variables|Default|GetMainMenu))))

(fn ConstructionScript)