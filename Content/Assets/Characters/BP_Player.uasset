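; Multiplayer player character Blueprint handling cosmetics, audio feedback and ability visual effects.
; BeginPlay applies saved customization from BP_GI and creates the local Esc menu; Tick updates an FPS readout and triggers authority-detected landing sounds.
; WASD state drives timer-looped footsteps through server/multicast events, with Shift quickening the pace.
; Timelines fade body and attached-item materials for invisibility and animate chromatic aberration, while SenseCollision toggles custom depth on CoreItems during X-ray mode.
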(event OnComponentBeginOverlap(SenseCollision)
  (params (OverlappedComponent :type Primitive%20Component%20Object%20Reference) (OtherActor :type Actor%20Object%20Reference) (OtherComp :type Primitive%20Component%20Object%20Reference) (OtherBodyIndex :type Integer) (bFromSweep :type Boolean) (SweepResult :type Hit%20Result%20Structure%20%28by%20ref%29))
  (if (Variables|Default|GetIsRentgenRender)
    (bind _ascore_item (Utilities|Casting|CastToCoreItem OtherActor))
    (Rendering|SetRenderCustomDepth (Variables|/Script/MyProject9.CollectableItem|GetMesh _ascore_item) true)))

(event OnComponentEndOverlap(SenseCollision)
  (params (OverlappedComponent :type Primitive%20Component%20Object%20Reference) (OtherActor :type Actor%20Object%20Reference) (OtherComp :type Primitive%20Component%20Object%20Reference) (OtherBodyIndex :type Integer))
  (if (Variables|Default|GetIsRentgenRender)
    (bind _ascore_item (Utilities|Casting|CastToCoreItem OtherActor))
    (Rendering|SetRenderCustomDepth (Variables|/Script/MyProject9.CollectableItem|GetMesh _ascore_item) false)))

(event Custom|PlayStepSound
  ;[1 1 1] Steps Sound mutherfucka
  (if (Math|Boolean|ANDBoolean (Variables|Default|GetIsNotInWebCam) (Variables|Default|GetbCanWalkingAndWatching) (not (Variables|Default|GetbInEscMenu)))
    (if (not (Variables|Default|GetReleasedAll))
      (if (Variables|Default|GetCurPlayingSoundStep)
        (if (not (Variables|Default|GetDoesLand))
          (Utilities|Time|SetTimerbyEvent (delegate Custom|PlayStepSound) 0.001 :!label _label)
          (else
            (Variables|Default|SetCurStepSound "/Game/Assets/Music/wova-zvuki-shagi-beg-po-betonnomu-polu__mp3cut_net_.wova-zvuki-shagi-beg-po-betonnomu-polu__mp3cut_net_")
            (if (> (Math|Vector|VectorLength (Pawn|Components|CharacterMovement|GetLastUpdateVelocity (Variables|Character|GetCharacterMovement))) 1e+02)
              (bind _returnvalue (Audio|SpawnSoundatLocation (Variables|Default|GetCurStepSound) (Transformation|GetActorLocation) "0, 0, 0" (* 0.05 2.0 (Variables|/Game/Assets/GameStuff/BP_GI.BP_GI_C|GetAudioMultiplayer (Variables|Default|GetInst))) 1.0 0.0 "/Game/Assets/Music/NewSoundAttenuation.NewSoundAttenuation" 0))
              (Variables|Default|SetSpawnedSoundStep _returnvalue))
            (Utilities|Time|SetTimerbyEvent (delegate Custom|PlayStepSound) (/ 0.45 (Variables|Default|GetDurationSteps)))))
        (else
          (goto _label))))))

(event Custom|PlayFallingSoundMulticast
  (Audio|PlaySoundatLocation "/Game/Assets/Music/Falling1.Falling1" (Transformation|GetActorLocation) "0, 0, 0" (* (Math|Float|Clamp(Float) (* (Variables|Default|GetVelocity) 0.001 0.2) 0.0 0.3) 2.0 (Variables|/Game/Assets/GameStuff/BP_GI.BP_GI_C|GetAudioMultiplayer (Variables|Default|GetInst)) 0.2) 1.0 0.0 "/Game/Assets/Music/NewSoundAttenuation.NewSoundAttenuation" 0 0))

(event Custom|GoodAttempClient
  ;[1 1 1] Generator Good Attemp Sound
  (Audio|SpawnSound2D "/Game/Assets/Music/GoodAttemptSound.GoodAttemptSound" (* 0.2 2.0 (Variables|/Game/Assets/GameStuff/BP_GI.BP_GI_C|GetAudioMultiplayer (Variables|Default|GetInst))) 1.0 0.0 0))

(event Custom|PlayRAbilityMulticast
  (params (NewParam :type Sound%20Wave%20Object%20Reference))
  (if (Variables|Default|GetIsPlayerOwner)
    (Audio|PlaySoundatLocation NewParam (Transformation|GetActorLocation) "0, 0, 0" (* 0.1 2.0 (Variables|/Game/Assets/GameStuff/BP_GI.BP_GI_C|GetAudioMultiplayer (Variables|Default|GetInst))) 1.0 0.0 "/Game/Assets/Music/NewSoundAttenuation.NewSoundAttenuation" 0 0)))

(event Custom|ReverceEverywhereMulticast
  (if (Variables|Default|GetIsPlayerOwner)
    (Class|UserView|RemoveIconfromPanel (Variables|Default|GetUserView) 2)
    (bind _newtrack_0 (Timeline|Invs Reverse)
      (:Update
        (for _array_element (Variables|Default|GetMatInstances)
          (Rendering|Material|SetScalarParameterValue _array_element "Opacity" _newtrack_0 :!class /Script/Engine.MaterialInstanceDynamic))
        (Rendering|Material|SetScalarParameterValue (Variables|Default|GetMat) "Opacity" _newtrack_0 :!class /Script/Engine.MaterialInstanceDynamic)))
    (else
      (Timeline|Invs Reverse))))

(event Custom|DeleteKADServer
  (bind _outactors (Actor|GetAllActorsOfClass "BP_Player_C"))
  (for _array_element _outactors
    (Class|Chel|DeleteKDATab _array_element (Variables|Default|GetIndex))))

(event Custom|PlayRAbilityServer
  (params (SoundWave :type Sound%20Wave%20Object%20Reference))
  (CallFunction|PlayRAbilityMulticast SoundWave))

(event Custom|InvisibleEverywhereMulticast
  (if (Variables|Default|GetHaveCreatedMatInstances)
    (bind _newtrack_0 (Timeline|Invs Play)
      (:Update
        (for _array_element (Variables|Default|GetMatInstances)
          (Rendering|Material|SetScalarParameterValue _array_element "Opacity" _newtrack_0 :!class /Script/Engine.MaterialInstanceDynamic))
        (Rendering|Material|SetScalarParameterValue (Variables|Default|GetMat) "Opacity" _newtrack_0 :!class /Script/Engine.MaterialInstanceDynamic)))
    (else
      (for _array_element_2 (Actor|GetAttachedActors true)
        (bind _asitem_custum_blueprint (Utilities|Casting|CastToItemCustumBlueprint _array_element_2))
        (Utilities|IsValid (Variables|/Game/Assets/Blueprint/Customization/ItemCustumBlueprint.ItemCustumBlueprint_C|GetStaticMesh _asitem_custum_blueprint)
          (:Is%20Valid
            (bind _returnvalue (Rendering|Material|CreateDynamicMaterialInstance (Variables|/Game/Assets/Blueprint/Customization/ItemCustumBlueprint.ItemCustumBlueprint_C|GetStaticMesh _asitem_custum_blueprint) 0 (Rendering|Material|GetMaterial (Variables|/Game/Assets/Blueprint/Customization/ItemCustumBlueprint.ItemCustumBlueprint_C|GetStaticMesh _asitem_custum_blueprint) 0) "None" :!class /Script/Engine.PrimitiveComponent))
            (Utilities|Array|Add (Variables|Default|GetMatInstances) _returnvalue))))
      (Variables|Default|SetHaveCreatedMatInstances true)
      (Timeline|Invs Play))))

(event Custom|PlayStoneThrowSoundMulticast
  ;[1 1 1] Stone Sound
  (Audio|PlaySoundatLocation "/Game/Assets/Music/StoneMusic1.StoneMusic1" (Transformation|GetActorLocation) "0, 0, 0" (* 0.1 2.0 (Variables|/Game/Assets/GameStuff/BP_GI.BP_GI_C|GetAudioMultiplayer (Variables|Default|GetInst))) 1.0 0.0 "/Game/Assets/Music/NewSoundAttenuation.NewSoundAttenuation" 0 0))

(event Custom|SpawnServer
  (params (Har :type Items%20Customization%20Struct%20Structure) (TShirt :type Items%20Customization%20Struct%20Structure) (Shirt :type Items%20Customization%20Struct%20Structure) (Accesori :type Items%20Customization%20Struct%20Structure))
  (bind _customizationchilds (Variables|Default|GetCustomizationChilds))
  (bind _poseablemeshcomp (Variables|Default|GetPoseableMeshComp))
  (bind _asbp_gi (Utilities|Casting|CastToBP_GI (Game|GetGameInstance)))
  (bind _outputitem (Default|AddItem _asbp_gi _poseablemeshcomp Har false))
  (Utilities|Array|Add _customizationchilds _outputitem)
  (bind _outputitem_2 (Default|AddItem _asbp_gi _poseablemeshcomp TShirt false))
  (Utilities|Array|Add _customizationchilds _outputitem_2)
  (bind _outputitem_3 (Default|AddItem _asbp_gi _poseablemeshcomp Shirt false))
  (Utilities|Array|Add _customizationchilds _outputitem_3)
  (bind _outputitem_4 (Default|AddItem _asbp_gi _poseablemeshcomp Accesori false))
  (Utilities|Array|Add _customizationchilds _outputitem_4))

(event Custom|Shagi_Server
  (params (1 :type Boolean) (2 :type Boolean) (3 :type Boolean) (4 :type Boolean))
  ;[1 1 1] Steps Sound mutherfucka
  (Variables|Default|SetReleasedAll false)
  (if (or (Math|Boolean|ANDBoolean (Math|Boolean|ANDBoolean (Math|Boolean|Equal(Boolean) 1 2) 1 2) (not 3) (not 4)) (Math|Boolean|ANDBoolean (Math|Boolean|ANDBoolean (Math|Boolean|Equal(Boolean) 3 4) 3 4) (not 1) (not 2)))
    (Variables|Default|SetCurPlayingSoundStep false)
    (CallFunction|StopLastSound)
    (elif (not (Variables|Default|GetCurPlayingSoundStep))
      (Variables|Default|SetCurPlayingSoundStep true)
      (CallFunction|ShagiMulticast))))

(event Custom|Shagi_Multicast
  ;[1 1 1] Steps Sound mutherfucka
  (CallFunction|PlayStepSound))

(event Custom|Govno
  (params (Syka :type Boolean) (Blyat :type Boolean) (Ebanii :type Boolean) (Rot :type Boolean))
  (bind _returnvalue (not Rot))
  (bind _returnvalue_2 (not Syka))
  (bind _returnvalue_3 (not Blyat))
  (bind _returnvalue_4 (not Ebanii))
  (bind _returnvalue_5 (Math|Boolean|ANDBoolean _returnvalue_2 _returnvalue_3 _returnvalue_4 _returnvalue))
  ;[1 1 1] Steps Sound mutherfucka
  (if (and (not (Variables|Default|GetDoesLand)) _returnvalue_5)
    (Variables|Default|SetReleasedAll true)
    (Variables|Default|SetCurPlayingSoundStep false)
    (CallFunction|StopLastSound)
    (elif (Math|Boolean|ORBoolean _returnvalue_5 (Math|Boolean|ANDBoolean (Math|Boolean|Equal(Boolean) Ebanii Rot) Ebanii Rot) (Math|Boolean|ANDBoolean (Math|Boolean|Equal(Boolean) Syka Blyat) Syka Blyat))
      (Variables|Default|SetCurPlayingSoundStep false)
      (CallFunction|StopLastSound)
      (else
        (Variables|Default|SetCurPlayingSoundStep true)))))

(event Custom|StopLastSound
  (bind _spawnedsoundstep (Variables|Default|GetSpawnedSoundStep))
  ;[1 1 1] Steps Sound mutherfucka
  (Utilities|IsValid _spawnedsoundstep
    (:Is%20Valid
      (Audio|Components|Audio|Stop _spawnedsoundstep))))

(event Custom|Change%20DurationSteps
  (params (Value :type Float%20%28single-precision%29))
  ;[1 1 1] Steps Sound mutherfucka
  (Variables|Default|SetDurationSteps Value))

(event Custom|PlayStoneHit_Multicast
  ;[1 1 1] Stone Sound
  (Audio|SpawnSoundatLocation "/Game/Assets/Music/Razrushenie.Razrushenie" (Transformation|GetActorLocation) "0, 0, 0" (* 0.1 2.0 (Variables|/Game/Assets/GameStuff/BP_GI.BP_GI_C|GetAudioMultiplayer (Variables|Default|GetInst))) 1.0 0.0 "/Game/Assets/Music/NewSoundAttenuation.NewSoundAttenuation" 0))

(event Custom|AddChromaticInvet_1
  ;[1 1 1] Bottle: ChromaticAbberation
  (bind _value_intencity (Timeline|Timeline_0 Play)
    (:Update
      (Variables|/Script/Engine.CameraComponent|SetPostProcessSettings (Variables|Default|GetCameraComp) (Utilities|Struct|MakePostProcessSettings _value_intencity)))))

(event Custom|RemoveChromaticInvet_1
  ;[1 1 1] Bottle: ChromaticAbberation
  (bind _value_intencity (Timeline|Timeline_0 ReverseFromEnd)
    (:Update
      (Variables|/Script/Engine.CameraComponent|SetPostProcessSettings (Variables|Default|GetCameraComp) (Utilities|Struct|MakePostProcessSettings _value_intencity)))))

(event EventTick
  (params (DeltaSeconds :type Float%20%28single-precision%29))
  (bind _userview (Variables|Default|GetUserView))
  (bind _charactermovement (Variables|Character|GetCharacterMovement))
  (Utilities|FlowControl|Sequence
    (:then_0
      (bind _output_get (Variables|Default|SetMyDelta (+ DeltaSeconds (Variables|Default|GetMyDelta))))
      (if (> _output_get 0.1)
        (Variables|Default|SetMyDelta 0.0)
        (Utilities|IsValid _userview
          (:Is%20Valid
            (Rendering|Components|TextRender|SetText (Variables|/Game/Assets/UI/UMG_UserView.UMG_UserView_C|GetTextBlock_FPS (.AsUMG%20User%20View (Utilities|Casting|CastToUMG_UserView _userview))) (Utilities|Text|FormatText "FPS  {int}" (Utilities|Text|ToText(Integer) (Math|Float|Ceil (/ 1.0 DeltaSeconds))))))
          (:Is%20Not%20Valid
            _)))
      (Networking|SwitchHasAuthority
        (:Authority
          (if (AI|Components|NavMovement|IsFalling _charactermovement)
            (Variables|Default|SetDoesLand false)
            (Variables|Default|SetVelocity (Math|Float|Absolute(Float) (.Z (Math|Vector|BreakVector (Pawn|Components|CharacterMovement|GetLastUpdateVelocity _charactermovement)))))
            (elif (not (Variables|Default|GetDoesLand))
              (Variables|Default|SetDoesLand true)
              (CallFunction|PlayFallingSoundMulticast))))))
    (:then_1
      (for _array_element (Variables|Default|GetRAbilityPanel)
        _))))

(event EventPickUpSound
  (Utilities|IsValid (Variables|Default|GetPickUpSoundEffect)
    (:Is%20Valid
      (Audio|Components|Audio|Stop (Variables|Default|GetPickUpSoundEffect)))
    (:Is%20Not%20Valid
      _))
  (bind _returnvalue (Audio|SpawnSound2D "/Game/Assets/Music/PickUpDouns.PickUpDouns" (* 1.0 2.0 (Variables|/Game/Assets/GameStuff/BP_GI.BP_GI_C|GetAudioMultiplayer (Variables|Default|GetInst))) 1.0 0.0 0))
  (Variables|Default|SetPickUpSoundEffect _returnvalue))

(event EventPlayArrowSound
  (Utilities|IsValid (Variables|Default|GetLastArrowSound)
    (:Is%20Valid
      (Audio|Components|Audio|Stop (Variables|Default|GetLastArrowSound)))
    (:Is%20Not%20Valid
      _))
  (bind _returnvalue (Audio|CreateSound2D "/Game/Assets/Music/arrowPromptSound.arrowPromptSound" (* 0.3 2.0 (Variables|/Game/Assets/GameStuff/BP_GI.BP_GI_C|GetAudioMultiplayer (Variables|Default|GetInst))) 1.0 0.0 0))
  (bind _output_get (Variables|Default|SetLastArrowSound _returnvalue))
  (Audio|Components|Audio|Play _output_get 0.0))

(event EventCameraTurnOff
  ;[1 1 1] Camera Sounds
  (Audio|PlaySound2D "/Game/Assets/Music/TV_Off_Sound.TV_Off_Sound" 1.0 1.0 0.0 0 0))

(event EventCameraSwitch
  ;[1 1 1] Camera Sounds
  (Utilities|IsValid (Variables|Default|GetSoundSwitch)
    (:Is%20Valid
      (Audio|Components|Audio|Stop (Variables|Default|GetSoundSwitch)))
    (:Is%20Not%20Valid
      _))
  (bind _returnvalue (Audio|SpawnSound2D "/Game/Assets/Music/CameraSwitch.CameraSwitch" (* 1.0 2.0 (Variables|/Game/Assets/GameStuff/BP_GI.BP_GI_C|GetAudioMultiplayer (Variables|Default|GetInst))) 1.0 0.0 0))
  (Variables|Default|SetSoundSwitch _returnvalue))

(event EventSpawnDeadSound
  ;[1 1 1] Dead and Wake Up Sound
  (Audio|SpawnSound2D "/Game/Assets/Music/DeadSound.DeadSound" (* 0.6 2.0 (Variables|/Game/Assets/GameStuff/BP_GI.BP_GI_C|GetAudioMultiplayer (Variables|Default|GetInst))) 1.0 0.0 0))

(event EventSpawnWakeUpSound
  ;[1 1 1] Dead and Wake Up Sound
  (Audio|SpawnSound2D "/Game/Assets/Music/WakeUp.WakeUp" (* 1.0 2.0 (Variables|/Game/Assets/GameStuff/BP_GI.BP_GI_C|GetAudioMultiplayer (Variables|Default|GetInst))) 1.0 0.0 0))

(event EventGoodAttempGeneratorSound
  ;[1 1 1] Generator Good Attemp Sound
  (CallFunction|GoodAttempClient))

(event EventCameraZoomin
  (bind _soundzoomingout (Variables|Default|GetSoundZoomingOut))
  ;[1 1 1] Camera Sounds
  (Utilities|IsValid _soundzoomingout
    (:Is%20Valid
      (Audio|Components|Audio|Stop _soundzoomingout))
    (:Is%20Not%20Valid
      _))
  (bind _returnvalue (Audio|SpawnSound2D "/Game/Assets/Music/CameraIn.CameraIn" (* 1.0 2.0 (Variables|/Game/Assets/GameStuff/BP_GI.BP_GI_C|GetAudioMultiplayer (Variables|Default|GetInst))) 1.0 0.0 0))
  (Variables|Default|SetSoundZoomingIn _returnvalue))

(event EventCameraZoomOut
  (bind _soundzoomingin (Variables|Default|GetSoundZoomingIn))
  ;[1 1 1] Camera Sounds
  (Utilities|IsValid _soundzoomingin
    (:Is%20Valid
      (Audio|Components|Audio|Stop _soundzoomingin))
    (:Is%20Not%20Valid
      _))
  (bind _returnvalue (Audio|SpawnSound2D "/Game/Assets/Music/CameraOut.CameraOut" (* 1.0 2.0 (Variables|/Game/Assets/GameStuff/BP_GI.BP_GI_C|GetAudioMultiplayer (Variables|Default|GetInst))) 1.0 0.0 0))
  (Variables|Default|SetSoundZoomingOut _returnvalue))

(event EventPlayStoneThrowSound
  ;[1 1 1] Stone Sound
  (CallFunction|PlayStoneThrowSoundMulticast))

(event EventReverceInvisibleEverywhere
  (CallFunction|ReverceEverywhereMulticast))

(event EventBeginPlay
  (bind _returnvalue (Rendering|Material|CreateDynamicMaterialInstance (Variables|Default|GetPoseableMeshComp) 0 "/Game/Assets/Models/Characters/material/CharacterMat.CharacterMat" "None" :!class /Script/Engine.PrimitiveComponent))
  (Variables|Default|SetMat _returnvalue)
  (Class|WidgetBlueprintLibrary|SetFocustoGameViewport)
  (bind _asbp_gi (Utilities|Casting|CastToBP_GI (Game|GetGameInstance)))
  (Utilities|FlowControl|Sequence
    (:then_0
      (Variables|Default|SetInst _asbp_gi)
      (if (== (Game|GetPlayerCharacter 0) self)
        (CallFunction|SpawnServer (Variables|/Game/Assets/GameStuff/BP_GI.BP_GI_C|GetPrevHat _asbp_gi) (Variables|/Game/Assets/GameStuff/BP_GI.BP_GI_C|GetPrevTShirt _asbp_gi) (Variables|/Game/Assets/GameStuff/BP_GI.BP_GI_C|GetPrevShirt _asbp_gi) (Variables|/Game/Assets/GameStuff/BP_GI.BP_GI_C|GetPrevAccesori _asbp_gi))
        (bind _returnvalue_2 (UserInterface|CreateWidget "/Game/Assets/UI/EscMenu.EscMenu_C" (.AsPlayer%20Controller (Utilities|Casting|CastToPlayerController (Pawn|GetController)))))
        (bind _output_get (Variables|Default|SetEscWidget _returnvalue_2))
        (Variables|/Script/MyProject9.EscapeMenu|SetPlayer _output_get self)
        (UserInterface|Viewport|AddtoViewport (Variables|Default|GetEscWidget) 0)
        (Widget|SetVisibility (Variables|Default|GetEscWidget) "Hidden")))
    (:then_1
      (if (== (Variables|/Script/MyProject9.GI|GetMaxPlayersCount _asbp_gi) 4)
        (bind _outactors (Actor|GetAllActorsOfClass "/Game/Assets/Blueprint/CanalizaciaAvaliableDoors.CanalizaciaAvaliableDoors_C"))
        (Rendering|SetActorHiddenInGame (Utilities|Array|Get(acopy) _outactors) true)
        (Collision|SetActorEnableCollision (Utilities|Array|Get(acopy) _outactors) false)))))

(event EventPofigKakNaz
  (params (SDJHfgActor :type Actor%20Object%20Reference))
  (bind _returnvalue (Transformation|GetActorLocation SDJHfgActor))
  (bind _returnvalue_2 (Game|GetPlayerController 0))
  (bind _screenposition (Class|GameplayStatics|ProjectWorldtoScreen _returnvalue_2 _returnvalue false))
  (Utilities|IsValid SDJHfgActor
    (:Is%20Valid
      (Variables|Default|SetScreenPosObj (Math|Vector2D|MakeVector2D (.x _screenposition) (.y _screenposition))))))

(event EventPlayStoneHit
  ;[1 1 1] Stone Sound
  (CallFunction|PlayStoneHitMulticast))

(event EventShowNoiseBlueprint
  (params (NewShow :type Boolean))
  (bind _asumg_web_cam_widget (Utilities|Casting|CastToUMG_WebCamWidget (Variables|Default|GetWebCamUI)))
  (if NewShow
    (Default|AddNoise _asumg_web_cam_widget)
    (else
      (Default|RemoveNoise _asumg_web_cam_widget))))

(event EventInvisibleEverywhere
  (CallFunction|InvisibleEverywhereMulticast))

(event EventPlayRAbilitySound
  (params (SoundWave :type Sound%20Wave%20Object%20Reference))
  (Audio|PlaySoundatLocation SoundWave (Transformation|GetActorLocation) "0, 0, 0" (* 0.1 2.0 (Variables|/Game/Assets/GameStuff/BP_GI.BP_GI_C|GetAudioMultiplayer (Variables|Default|GetInst))) 1.0 0.0 "/Game/Assets/Music/NewSoundAttenuation.NewSoundAttenuation" 0 0))

(event EventAddChromaticAbberation
  ;[1 1 1] Medkit: ChromaticAbberation
  (bind _value_intencity (Timeline|Chromatic PlayFromStart)
    (:Update
      (Variables|/Script/Engine.CameraComponent|SetPostProcessSettings (Variables|Default|GetCameraComp) (Utilities|Struct|MakePostProcessSettings _value_intencity)))))

(event Input|KeyboardEvents|W
  (params (Key :type Key%20Structure :default "None"))
  ;[1 1 1] Steps Sound mutherfucka
  (:Pressed
    (Variables|Default|SetPressedW true)
    (CallFunction|ShagiServer (Variables|Default|GetPressedW) (Variables|Default|GetPressedS) (Variables|Default|GetPressedA) (Variables|Default|GetPressedD)))
  (:Released
    (Variables|Default|SetPressedW false)
    (CallFunction|Govno (Variables|Default|GetPressedW) (Variables|Default|GetPressedS) (Variables|Default|GetPressedA) (Variables|Default|GetPressedD))))

(event Input|KeyboardEvents|S
  (params (Key :type Key%20Structure :default "None"))
  ;[1 1 1] Steps Sound mutherfucka
  (:Pressed
    (Variables|Default|SetPressedS true)
    (CallFunction|ShagiServer (Variables|Default|GetPressedW) (Variables|Default|GetPressedS) (Variables|Default|GetPressedA) (Variables|Default|GetPressedD)))
  (:Released
    (Variables|Default|SetPressedS false)
    (CallFunction|Govno (Variables|Default|GetPressedW) (Variables|Default|GetPressedS) (Variables|Default|GetPressedA) (Variables|Default|GetPressedD))))

(event Input|KeyboardEvents|A
  (params (Key :type Key%20Structure :default "None"))
  ;[1 1 1] Steps Sound mutherfucka
  (:Pressed
    (Variables|Default|SetPressedA true)
    (CallFunction|ShagiServer (Variables|Default|GetPressedW) (Variables|Default|GetPressedS) (Variables|Default|GetPressedA) (Variables|Default|GetPressedD)))
  (:Released
    (Variables|Default|SetPressedA false)
    (CallFunction|Govno (Variables|Default|GetPressedW) (Variables|Default|GetPressedS) (Variables|Default|GetPressedA) (Variables|Default|GetPressedD))))

(event Input|KeyboardEvents|D
  (params (Key :type Key%20Structure :default "None"))
  ;[1 1 1] Steps Sound mutherfucka
  (:Pressed
    (Variables|Default|SetPressedD true)
    (CallFunction|ShagiServer (Variables|Default|GetPressedW) (Variables|Default|GetPressedS) (Variables|Default|GetPressedA) (Variables|Default|GetPressedD)))
  (:Released
    (Variables|Default|SetPressedD false)
    (CallFunction|Govno (Variables|Default|GetPressedW) (Variables|Default|GetPressedS) (Variables|Default|GetPressedA) (Variables|Default|GetPressedD))))

(event Input|KeyboardEvents|LeftShift
  (params (Key :type Key%20Structure :default "None"))
  ;[1 1 1] Steps Sound mutherfucka
  (:Pressed
    (CallFunction|ChangeDurationSteps 1.6))
  (:Released
    (CallFunction|ChangeDurationSteps 1.0)))

(fn ConstructionScript)