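; BP_Player_Menu is the main menu player actor, which has the game instance show the main menu on start.
; BeginPlay also finds the first Menu_Door in the level and records its start location.
; The Open event plays a timeline that offsets the door vertically from that location while yawing this actor.
; Tick continuously rotates the camera by a fixed world-space step, unscaled by delta time.
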(event Custom|Open
  (bind _startlocation (Variables|Default|GetStartLocation))
  (bind (_direction _up _newtrack_1) (Timeline|Timeline_0 PlayFromStart)
    (:Update
      (Transformation|SetActorLocation (Variables|/Game/Assets/Blueprint/Menu_Door.Menu_Door_C|GetStaticMesh (Variables|Default|GetMenuDoor)) (Math|Vector|MakeVector (.x _startlocation) (.y _startlocation) (+ _up (.z _startlocation))) false false)
      (Transformation|SetActorRotation (Math|Rotator|MakeRotator 0.0 0.0 _newtrack_1)))))

(event EventBeginPlay
  (bind _asbp_gi (Utilities|Casting|CastToBP_GI (Game|GetGameInstance)))
  (Default|ShowMainMenu _asbp_gi)
  (bind _outactors (Actor|GetAllActorsOfClass "/Game/Assets/Blueprint/Menu_Door.Menu_Door_C"))
  (bind _output_get (Variables|Default|SetMenuDoor (Utilities|Array|Get(acopy) _outactors)))
  (Variables|Default|SetStartLocation (Transformation|GetActorLocation (Variables|/Game/Assets/Blueprint/Menu_Door.Menu_Door_C|GetStaticMesh _output_get))))

(event EventTick
  (params (DeltaSeconds :type Float%20%28single-precision%29))
  (Transformation|AddWorldRotation (Variables|Default|GetCamera) "0,10.000000, 0" false false))

(fn ConstructionScript)