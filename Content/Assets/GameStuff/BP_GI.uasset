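; Game instance that runs multiplayer sessions, menu screens and saved player preferences, including cosmetics.
; Hosts through Advanced Sessions with a nickname-plus-number GAMENAME, and joins via invite, ID match or any non-full session.
; Triggers the menu character's Open before a timed listen-server travel or join.
; AddItem and RemoveItem attach or detach cosmetic actors and track each slot, which QuitGame saves to the Preset slot and Init reloads.
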(event Custom|QuitGame
  (params (PrevWidget :type User%20Widget%20Object%20Reference))
  (bind _playercustomizationpreset (Variables|Default|GetPlayerCustomizationPreset))
  (Variables|/Game/Assets/GameStuff/ChelPreset.ChelPreset_C|SetAudioMultiplayer _playercustomizationpreset (Variables|Default|GetAudioMultiplayer))
  (Variables|/Game/Assets/GameStuff/ChelPreset.ChelPreset_C|SetAccessori _playercustomizationpreset (Variables|Default|GetPrevAccesori))
  (Variables|/Game/Assets/GameStuff/ChelPreset.ChelPreset_C|SetHat _playercustomizationpreset (Variables|Default|GetPrevHat))
  (Variables|/Game/Assets/GameStuff/ChelPreset.ChelPreset_C|SetTShirt _playercustomizationpreset (Variables|Default|GetPrevTShirt))
  (Variables|/Game/Assets/GameStuff/ChelPreset.ChelPreset_C|SetShirt _playercustomizationpreset (Variables|Default|GetPrevShirt))
  (Variables|/Game/Assets/GameStuff/ChelPreset.ChelPreset_C|SetSensetivity _playercustomizationpreset (Variables|Default|GetSensetivity))
  (Variables|/Game/Assets/GameStuff/ChelPreset.ChelPreset_C|SetNickName _playercustomizationpreset (Variables|Default|GetNickName))
  (Variables|/Game/Assets/GameStuff/ChelPreset.ChelPreset_C|SetIsEnPrompt _playercustomizationpreset (Variables|Default|GetbIsEnabledPrompt))
  (SaveGame|SaveGametoSlot _playercustomizationpreset "Preset")
  (Utilities|IsValid PrevWidget
    (:Is%20Valid
      (Widget|RemovefromParent PrevWidget))
    (:Is%20Not%20Valid
      _))
  (Game|QuitGame (Game|GetPlayerController 0) "Quit" false))

(event Custom|OpenLevel
  (Game|OpenLevel(byName) "MainLevel" true "listen"))

(event Custom|JoinServer
  (params (Widget :type User%20Widget%20Object%20Reference) (IsWithID :type Boolean))
  (bind _asumg_main_menu (Utilities|Casting|CastToUMG_MainMenu Widget))
  (Variables|Default|SetMenuWidget _asumg_main_menu)
  (bind _results (|FindSessionsAdvanced (Game|GetPlayerController 0) 1000 false "ClientServersOnly" 0 false false false)
    (:OnSuccess
      (bind _output_get (Variables|Default|SetSessions _results))
      (if (!= (Utilities|Array|Length _output_get) 0)
        (bind _array_element (Utilities|Array|ForEachLoopwithBreak _output_get)
          (:LoopBody
            (if IsWithID
              (bind _extrasettings (Class|AdvancedSessionsLibrary|GetExtraSettings _array_element))
              (bind _settingvalue (Class|AdvancedSessionsLibrary|GetSessionPropertyString _extrasettings "GAMENAME")
                (:Found
                  (if (Utilities|Enum|Equal(Enum) (Utilities|String|ToString(Text) (Class|EditableText|GetText (Variables|/Script/MyProject9.MainMenu|GetServerConnectID (Variables|Default|GetMenuWidget)))) _settingvalue)
                    (if (< (Class|FindSessionsCallbackProxy|GetCurrentPlayers _array_element) (Class|FindSessionsCallbackProxy|GetMaxPlayers _array_element)) :!label _label
                      (Development|PrintString (Utilities|String|ToString(Integer) (Class|FindSessionsCallbackProxy|GetMaxPlayers _array_element)))
                      (Variables|Default|SetMaxPlayersCount (Class|FindSessionsCallbackProxy|GetMaxPlayers _array_element))
                      (bind _output_get_2 (Variables|Default|SetSessionToConnect _array_element))
                      (Development|PrintString (Class|AdvancedSessionsLibrary|GetSessionIDasString _output_get_2))
                      (bind _asbp_player_menu_test (Utilities|Casting|CastToBP_Player_MenuTest (Game|GetPlayerCharacter 0)))
                      (Default|Open _asbp_player_menu_test)
                      (Utilities|Time|SetTimerbyEvent (delegate Custom|JoinLevel) 5.0)))))
              (else
                (goto _label)))))
        (else
          (Default|Failed (Variables|Default|GetMenuWidget) :!label _label_2))))
    (:OnFailure
      (goto _label_2))))

(event Custom|DestroyServer
  (params (Player :type Player%20Controller%20Object%20Reference) (PrevWidget :type User%20Widget%20Object%20Reference))
  (|DestroySession Player
    (:OnSuccess
      (Game|OpenLevel(byName) "MENU"))))

(event Custom|ShowMainMenu
  (params (PrevWidget :type User%20Widget%20Object%20Reference))
  (bind _returnvalue (Game|GetPlayerController 0))
  (Utilities|IsValid PrevWidget
    (:Is%20Valid
      (Widget|RemovefromParent PrevWidget))
    (:Is%20Not%20Valid
      _))
  (bind _returnvalue_2 (UserInterface|CreateWidget "/Game/Assets/UI/UMG_MainMenu.UMG_MainMenu_C" _returnvalue))
  (UserInterface|Viewport|AddtoViewport _returnvalue_2 0)
  (Variables|/Script/Engine.PlayerController|SetbShowMouseCursor _returnvalue true)
  (bind _asbp_player_menu_test (Utilities|Casting|CastToBP_Player_MenuTest (Game|GetPlayerCharacter 0)))
  (Variables|/Game/Assets/Characters/BP_Player_MenuTest.BP_Player_MenuTest_C|SetMainMenu _asbp_player_menu_test _returnvalue_2))

(event Custom|ShowJoinServer
  (params (PrevWidget :type User%20Widget%20Object%20Reference))
  (Utilities|IsValid PrevWidget
    (:Is%20Valid
      (Widget|RemovefromParent PrevWidget))
    (:Is%20Not%20Valid
      _))
  (bind _returnvalue (UserInterface|CreateWidget "/Game/Assets/UI/JoinScreen.JoinScreen_C" (Game|GetPlayerController 0)))
  (UserInterface|Viewport|AddtoViewport _returnvalue 0))

(event Custom|JoinLevel
  (|JoinSession (Game|GetPlayerController 0) (stale Custom|JoinServer _output_get_2)
    (:OnFailure
      (bind _asbp_player_menu_test (Utilities|Casting|CastToBP_Player_MenuTest (Game|GetPlayerCharacter 0))
        (:then
          (Default|Close _asbp_player_menu_test))
        (:CastFailed
          _))
      (Default|Failed (Variables|Default|GetMenuWidget))
      (Utilities|Array|ForEachLoopwithBreak (stale Custom|JoinServer _output_get)) ; enters at Break
    )))

(event Custom|CreateServer
  (params (Widget :type User%20Widget%20Object%20Reference))
  (bind _returnvalue (Math|Random|RandomIntegerinRange 100000000 999999999))
  (bind _nickname (Variables|Default|GetNickName))
  (bind _returnvalue_2 (Utilities|String|ToString(Text) _nickname))
  (bind _returnvalue_3 (Utilities|String|ToString(Integer) _returnvalue))
  (bind _returnvalue_4 (Utilities|String|Append _returnvalue_2 _returnvalue_3))
  (Utilities|IsValid Widget
    (:Is%20Valid
      _)
    (:Is%20Not%20Valid
      _))
  (|AdvancedSession (Utilities|Array|MakeArray (Class|AdvancedSessionsLibrary|MakeLiteralSessionPropertyString "GAMENAME" _returnvalue_4)) (Game|GetPlayerController 0) (Variables|Default|GetMaxPlayersCount) 0 false true false true true false false false true
    (:OnSuccess
      (Variables|Default|SetSessionID _returnvalue_4)
      (bind _asbp_player_menu_test (Utilities|Casting|CastToBP_Player_MenuTest (Game|GetPlayerCharacter 0)))
      (Default|Open _asbp_player_menu_test)
      (Utilities|Time|SetTimerbyEvent (delegate Custom|OpenLevel) 5.0))))

(event EventInit
  (Class|WidgetBlueprintLibrary|SetFocustoGameViewport)
  (bind _returnvalue (SaveGame|CreateSaveGameObject "/Game/Assets/GameStuff/ChelPreset.ChelPreset_C"))
  (Variables|Default|SetPlayerCustomizationPreset _returnvalue)
  (bind _returnvalue_2 (SaveGame|LoadGamefromSlot "Preset"))
  (bind _aschel_preset (Utilities|Casting|CastToChelPreset _returnvalue_2))
  (bind _output_get (Variables|Default|SetPlayerCustomizationPreset _aschel_preset))
  (Variables|Default|SetPrevHat (Variables|/Game/Assets/GameStuff/ChelPreset.ChelPreset_C|GetHat _output_get))
  (Variables|Default|SetPrevShirt (Variables|/Game/Assets/GameStuff/ChelPreset.ChelPreset_C|GetShirt _output_get))
  (Variables|Default|SetPrevTShirt (Variables|/Game/Assets/GameStuff/ChelPreset.ChelPreset_C|GetTShirt _output_get))
  (Variables|Default|SetPrevAccesori (Variables|/Game/Assets/GameStuff/ChelPreset.ChelPreset_C|GetAccessori _output_get))
  (Variables|Default|SetSensetivity (Variables|/Game/Assets/GameStuff/ChelPreset.ChelPreset_C|GetSensetivity _output_get))
  (Variables|Default|SetNickName (Variables|/Game/Assets/GameStuff/ChelPreset.ChelPreset_C|GetNickName _output_get))
  (Variables|Default|SetAudioMultiplayer (Variables|/Game/Assets/GameStuff/ChelPreset.ChelPreset_C|GetAudioMultiplayer _output_get))
  (Variables|Default|SetbIsEnabledPrompt (Variables|/Game/Assets/GameStuff/ChelPreset.ChelPreset_C|GetIsEnPrompt _output_get)))

(event EventOnSessionInviteAccepted
  (params (LocalPlayerNum :type Integer) (PersonInvited :type BP%20Unique%20Net%20Id%20Structure) (SessionToJoin :type Blueprint%20Session%20Result%20Structure%20%28by%20ref%29))
  (bind _output_get (Variables|Default|SetSessionToConnect SessionToJoin))
  (Variables|Default|SetMaxPlayersCount (Class|FindSessionsCallbackProxy|GetMaxPlayers _output_get))
  (bind _asbp_player_menu_test (Utilities|Casting|CastToBP_Player_MenuTest (Game|GetPlayerCharacter 0)))
  (Default|Open _asbp_player_menu_test)
  (Utilities|Time|SetTimerbyEvent (delegate Custom|JoinLevel) 5.0))

(event EventOnSessionInviteReceived
  (params (LocalPlayerNum :type Integer) (PersonInviting :type BP%20Unique%20Net%20Id%20Structure) (AppId :type String) (SessionToJoin :type Blueprint%20Session%20Result%20Structure%20%28by%20ref%29))
  (Development|PrintString "Hello"))

(fn RemoveItem
  (params (Type :type Integer))
  (bind _outactors (Actor|GetAllActorsOfClass "/Game/Assets/Blueprint/Customization/ItemCustumBlueprint.ItemCustumBlueprint_C"))
  (for _array_element _outactors
    (if (== (Variables|/Game/Assets/Blueprint/Customization/ItemCustumBlueprint.ItemCustumBlueprint_C|GetType _array_element) Type)
      (switch int (Variables|/Game/Assets/Blueprint/Customization/ItemCustumBlueprint.ItemCustumBlueprint_C|GetType _array_element)
        (:0
          (Variables|Default|SetPrevHat ""))
        (:1
          (Variables|Default|SetPrevTShirt ""))
        (:2
          (Variables|Default|SetPrevShirt ""))
        (:3
          (Variables|Default|SetPrevAccesori "")))
      (Default|DetatchEvent _array_element))))

(fn AddItem
  (params (Component :type Scene%20Component%20Object%20Reference) (Struct :type Items%20Customization%20Struct%20Structure) (DoesHaveText :type Boolean) (OwnerItem :type BP%20Player%20Object%20Reference))
  (bind (_isopen _type _image _nameitem _meshitem _transformitem _socketname) (Utilities|Struct|BreakItemsCustomizationStruct Struct))
  (if (Utilities|IsValid _meshitem)
    (bind _returnvalue (Game|SpawnActorfromClass "/Game/Assets/Blueprint/Customization/ItemCustumBlueprint.ItemCustumBlueprint_C" _transformitem "Undefined" OwnerItem _type 0))
    (Components|StaticMesh|SetStaticMesh (Variables|/Game/Assets/Blueprint/Customization/ItemCustumBlueprint.ItemCustumBlueprint_C|GetStaticMesh _returnvalue) _meshitem)
    (Transformation|AttachComponentToComponent _returnvalue Component _socketname "KeepRelative" "KeepRelative" "KeepRelative" true)
    (if DoesHaveText
      _
      (else
        (switch int _type
          (:0
            (Variables|Default|SetPrevHat Struct))
          (:1
            (Variables|Default|SetPrevTShirt Struct))
          (:2
            (Variables|Default|SetPrevShirt Struct))
          (:3
            (Variables|Default|SetPrevAccesori Struct))))))
  (return _returnvalue))