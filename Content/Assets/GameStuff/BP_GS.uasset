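; BP_GS is a game state whose only live logic sets up customized characters for match winners.
; SpawnCustomizationChels loops over PlayersTransform, finds the BP_PlayerContr whose Index matches WinnersIndex for that slot, and calls GetCustomizationPreset with the slot index.
; A code-terminal puzzle (random five-digit code note, spawned digit actors, code check, status lamp) remains as disconnected logic that never runs, leaving its events empty.
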(event Custom|AddNumToTerminal
  (params (Number :type Integer)))

(event Custom|DeleteLastNumber)

(event Custom|CheckCode)

(event Custom|ChangeMaterialLamp
  (params (CodeColor :type Integer)))

(event Custom|SpawnNote_1)

(event EventBeginPlay)

(event EventSpawnCustomizationChels
  (bind _asbp_gs (Utilities|Casting|CastToBP_GS (Game|GetGameState)))
  (for (_ _array_index) (Variables|Default|GetPlayersTransform)
    (bind _outactors (Actor|GetAllActorsOfClass "/Game/Assets/Characters/BP_PlayerContr.BP_PlayerContr_C"))
    (bind _array_element (Utilities|Array|ForEachLoopwithBreak _outactors :!label _label)
      (:LoopBody
        (if (== (Variables|/Script/MyProject9.BP_PlayerController|GetIndex _array_element) (Utilities|Array|Get(acopy) (Variables|/Script/MyProject9.GS|GetWinnersIndex _asbp_gs) _array_index))
          (Default|GetCustomizationPreset _array_element _array_index)
          (Development|PrintString "Spawn")
          (goto _label Break))))))

(event EventTick
  (params (DeltaSeconds :type Float%20%28single-precision%29)))

(fn ConstructionScript)